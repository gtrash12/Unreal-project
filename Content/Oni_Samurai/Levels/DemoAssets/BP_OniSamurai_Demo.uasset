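; BP_OniSamurai_Demo is a demo actor for the Oni Samurai asset, controlled from the keyboard.
; BeginPlay enables input from the first player controller, and R flip-flops a slow yaw spin on and off through the RotatingMovement component.
; Space Bar increments the AnimPlayed index up to 12, then wraps it to zero; nothing in this Blueprint's graphs consumes that value.
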(event EventBeginPlay
  (Input|EnableInput (Game|GetPlayerController 0)))

(event Collision|EventActorBeginOverlap
  (params (OtherActor :type Actor%20Object%20Reference)))

(event EventTick
  (params (DeltaSeconds :type Float%20%28single-precision%29)))

(event Input|KeyboardEvents|SpaceBar
  (params (Key :type Key%20Structure))
  (:Pressed
    (if (< (Variables|Default|GetAnimPlayed) 12)
      (Math|Integer|IncrementInt (Variables|Default|GetAnimPlayed))
      (else
        (Variables|Default|SetAnimPlayed 0)))))

(event Input|KeyboardEvents|R
  (params (Key :type Key%20Structure))
  (bind _rotatingmovement (Variables|Default|GetRotatingMovement))
  (:Pressed
    (Utilities|FlowControl|FlipFlop
      (:A
        (Variables|/Script/Engine.RotatingMovementComponent|SetRotationRate _rotatingmovement "0,5.000000, 0"))
      (:B
        (Variables|/Script/Engine.RotatingMovementComponent|SetRotationRate _rotatingmovement "0, 0, 0")))))

(fn ConstructionScript)