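; Epic treasure chest Blueprint that plays a one-time unlock sequence when something first overlaps its box trigger.
; The sequence chains diegetic sound, skeletal animation and timeline-driven lid opening, with optional ethereal and melodic audio, particles and light fade-in, then auto-closes and sets IsUnlocked.
; Once unlocked, overlap begin and end play and reverse a separate lid timeline.
; The construction script sets light color, zeroes intensity and optionally shows interior meshes.
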(event OnComponentEndOverlap(Box)
  (params (OverlappedComponent :type Primitive%20Component%20Object%20Reference) (OtherActor :type Actor%20Object%20Reference) (OtherComp :type Primitive%20Component%20Object%20Reference) (OtherBodyIndex :type Integer))
  ;[1 1 1] Open and Close if Unlocked
  (if (Variables|Default|GetisUnlocked)
    (bind _cme_open (Timeline|Open%20and%20CloseLid%20Unlocked Reverse)
      (:Update
        (Transformation|SetRelativeRotation (Variables|Default|GetSM_Lid) (Math|Rotator|MakeRotator _cme_open 0.0 0.0) false false)))))

(event OnComponentBeginOverlap(Box)
  (params (OverlappedComponent :type Primitive%20Component%20Object%20Reference) (OtherActor :type Actor%20Object%20Reference) (OtherComp :type Primitive%20Component%20Object%20Reference) (OtherBodyIndex :type Integer) (bFromSweep :type Boolean) (SweepResult :type Hit%20Result%20Structure%20%28by%20ref%29))
  (bind _sm_base (Variables|Default|GetSM_Base))
  (bind _returnvalue (Transformation|GetWorldLocation _sm_base))
  (if (Variables|Default|GetisUnlocked)
    ;[1 1 1] Open and Close if Unlocked
    (Audio|PlaySoundatLocation "/Game/Heroic_Chests_Volume_1/Audio/ECV1_Common_Clasp_Cue.ECV1_Common_Clasp_Cue" (Transformation|GetWorldLocation (Variables|Default|GetSM_Base)) "0, 0, 0" 1.0 1.0 0.0 "/Game/Heroic_Chests_Volume_1/Audio/Attenuation_Basic_SA.Attenuation_Basic_SA")
    (bind _cme_open (Timeline|Open%20and%20CloseLid%20Unlocked Play)
      (:Update
        (Transformation|SetRelativeRotation (Variables|Default|GetSM_Lid) (Math|Rotator|MakeRotator _cme_open 0.0 0.0) false false)))
    (else
      ;[1 1 1] Implement User Variables
      (Utilities|FlowControl|DoOnce false
        (:Completed
          (Audio|PlaySoundatLocation "/Game/Heroic_Chests_Volume_1/Audio/ECV1_Epic_Diagetic_Cue.ECV1_Epic_Diagetic_Cue" _returnvalue "0, 0, 0" 1.0 1.0 0.0 "/Game/Heroic_Chests_Volume_1/Audio/Attenuation_Basic_SA.Attenuation_Basic_SA")
          (if (Variables|Default|GetEthereal)
            (Audio|PlaySoundatLocation "/Game/Heroic_Chests_Volume_1/Audio/ECV1_Epic_Ethereal_Cue.ECV1_Epic_Ethereal_Cue" _returnvalue "0, 0, 0" 1.0 1.0 0.0 "/Game/Heroic_Chests_Volume_1/Audio/Attenuation_Basic_SA.Attenuation_Basic_SA")
            (Utilities|FlowControl|Delay 0.3))
          (Components|Animation|PlayAnimation (Variables|Default|GetSKM_Animation) "/Game/Heroic_Chests_Volume_1/Animations/ECV1_Epic_Anim.ECV1_Epic_Anim" false)
          (Utilities|FlowControl|Delay 6.0)
          (if (Variables|Default|Getparticles)
            (Components|Activation|Activate (Variables|Default|GetECV1_Epic) false))
          (Utilities|FlowControl|Delay 1.0)
          (if (Variables|Default|GetMelodic)
            (Audio|PlaySound2D "/Game/Heroic_Chests_Volume_1/Audio/ECV1_Epic_Melodic_Cue.ECV1_Epic_Melodic_Cue")
            ;[1 1 1] Open Lid
            (bind (_direction _cme_open_2 _lightintensity) (Timeline|Open_Lid PlayFromStart)
              (:Update
                (Transformation|SetRelativeRotation (Variables|Default|GetSM_Lid) (Math|Rotator|MakeRotator _cme_open_2 0.0 0.0) false false)
                (if (Variables|Default|Getlight)
                  (Rendering|Components|Light|SetIntensity (Variables|Default|GetPointLight) (Math|Float|Lerp 0.0 (Variables|Default|GetIntensity) _lightintensity))
                  (Utilities|FlowControl|DoOnce false
                    (:Completed
                      (Audio|PlaySoundatLocation "/Game/Heroic_Chests_Volume_1/Audio/ECV1_Common_Clasp_Cue.ECV1_Common_Clasp_Cue" (Transformation|GetWorldLocation (Variables|Default|GetSM_Base)) "0, 0, 0" 1.0 1.0 0.0 "/Game/Heroic_Chests_Volume_1/Audio/Attenuation_Basic_SA.Attenuation_Basic_SA")))))
              (:Finished
                ;[1 1 1] Close Lid
                (Utilities|FlowControl|DoOnce false
                  (:Completed
                    (Variables|Default|SetIntensity 0.0)
                    (Utilities|FlowControl|Delay 1e+01)
                    (bind _cme_open_3 (Timeline|Close%20Lid PlayFromStart)
                      (:Update
                        (Transformation|SetRelativeRotation (Variables|Default|GetSM_Lid) (Math|Rotator|MakeRotator _cme_open_3 0.0 0.0) false false))
                      (:Finished
                        (Variables|Default|SetisUnlocked true)))))))
            (else
              (Timeline|Open_Lid PlayFromStart))))))))

(fn ConstructionScript
  (bind _pointlight (Variables|Default|GetPointLight))
  (Rendering|Components|Light|SetLightColor _pointlight (Variables|Default|GetLight%20Color) true)
  (Rendering|Components|Light|SetIntensity _pointlight 0.0)
  (if (Variables|Default|GetInterior)
    (Rendering|SetVisibility (Variables|Default|GetSM_Base_Interior) true false)
    (Rendering|SetVisibility (Variables|Default|GetSM_Lid_Interior) true false)))