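; Camera actor that follows a Target actor with a spring-arm camera, interpolating location and rotation every tick after the Target ticks.
; A Camera-channel trace beside the Target shifts the follow point sideways to avoid walls, with a DoOnce restoring offsets once clear.
; Rotation follows control rotation, but above a speed threshold without mouse or left-stick input it eases toward facing the Target and sets control rotation to that look-at direction.
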(event EventBeginPlay
  (bind _target (Variables|Default|GetTarget))
  (bind _returnvalue (Transformation|GetActorLocation _target))
  (bind _mesh (Variables|/Script/Engine.Character|GetMesh _target))
  (bind _returnvalue_2 (Transformation|GetSocketLocation _mesh "camera_following_socket"))
  (bind _returnvalue_3 (- _returnvalue_2 _returnvalue))
  (Actor|Tick|AddTickPrerequisiteActor (Variables|Default|GetTarget))
  (Utilities|FlowControl|Delay 2.0)
  (Variables|Default|Setoriginal_offset (Math|Vector|MakeVector 0.0 (.y _returnvalue_3) (* (.z _returnvalue_3) -1.0))))

(event EventTick
  (params (DeltaSeconds :type Float%20%28single-precision%29))
  (bind _returnvalue (Game|GetPlayerController 0))
  (bind _target (Variables|Default|GetTarget))
  (bind _camera (Variables|Default|GetCamera))
  (bind _target_2 (Variables|Default|GetTarget))
  (bind _target_3 (Variables|Default|GetTarget))
  (bind _returnvalue_2 (Transformation|GetWorldLocation _camera))
  (bind (_stickx _sticky) (Class|PlayerController|GetInputAnalogStickState _returnvalue "CAS_LeftStick"))
  (bind _returnvalue_3 (Transformation|GetActorLocation _target_2))
  (bind (_deltax _deltay) (Class|PlayerController|GetInputMouseDelta _returnvalue))
  (bind _returnvalue_4 (Transformation|GetActorLocation _target))
  (bind _returnvalue_5 (Math|Rotator|FindLookatRotation _returnvalue_2 _returnvalue_4))
  (Utilities|FlowControl|Sequence
    (:then_0
      ;[1 1 1] 카메라 벽 밖으로 안나가게
      (bind (_outhit _returnvalue_6) (Collision|LineTraceByChannel (+ (* (Math|Vector|GetRightVector (Transformation|GetActorRotation (Variables|Default|GetTarget))) 6e+01) _returnvalue_3) _returnvalue_3 "TraceTypeQuery2" false 0 "None"))
      (if (and _returnvalue_6 (.bBlockingHit (Collision|BreakHitResult _outhit)))
        (Variables|Default|Setlocation_offset (Math|Vector|MakeVector 0.0 (- (Math|Vector|Distance(Vector) (.Location (Collision|BreakHitResult _outhit)) _returnvalue_3) 6e+01) 0.0))
        (goto _label Reset)
        (else
          (Utilities|FlowControl|DoOnce true :!label _label
            (:Completed
              (Variables|Default|Setlocation_offset (Math|Vector|MakeVector 0.0 0.0 0.0))
              (Variables|/Script/Engine.SpringArmComponent|SetSocketOffset (Variables|Default|GetSpringArm) "0,20.000000, 0"))))))
    (:then_1
      (Transformation|SetActorLocation (Math|Interpolation|VInterpTo (Transformation|GetActorLocation) (+ (Transformation|GetActorLocation _target_3) (* (Math|Vector|GetRightVector (Transformation|GetActorRotation (Variables|Default|GetTarget))) (.y (+ (Variables|Default|Getlocation_offset) "0, 0, 0")))) DeltaSeconds 1e+01) false false)
      (if (< (Math|Vector|VectorLength (Transformation|GetVelocity _target_3)) 2e+03)
        (Transformation|SetActorRotation (Math|Interpolation|RInterpTo (Transformation|GetActorRotation) (Pawn|GetControlRotation (Variables|Default|GetTarget) :!class /Script/Engine.Pawn) DeltaSeconds 1e+01) :!label _label_2)
        (elif (Math|Boolean|ANDBoolean (== _deltax 0.0) (== _deltay 0.0) (== _stickx 0.0) (== _sticky 0.0))
          ;[1 1 1] 캐릭터 속도 임계치 초과시 컨트롤 로테이션이 아니라 캐릭터를 바라보는 방향으로 카메라 보간 후 컨트롤 로테이션을 맞춤
          (Transformation|SetActorRotation (Math|Interpolation|RInterpTo (Transformation|GetActorRotation) _returnvalue_5 DeltaSeconds 2.5))
          (Pawn|SetControlRotation (Game|GetPlayerController 0) _returnvalue_5)
          (else
            (goto _label_2)))))))

(fn ConstructionScript)