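; Explosive trap actor that goes off when something overlaps its cylinder, damaging that actor.
; On the server, the overlap fires a multicast that plays an explosion sound and particle effect, then sends a damage message to the overlapping actor with the trap as causer.
; Getter functions, apparently from a shared character/combat interface, return fixed defaults or the trap's damage data.
; BeginPlay adds the first player pawn as a tick prerequisite.
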(event OnComponentBeginOverlap(Cylinder)
  (params (OverlappedComponent :type Primitive%20Component%20Object%20Reference) (OtherActor :type Actor%20Object%20Reference) (OtherComp :type Primitive%20Component%20Object%20Reference) (OtherBodyIndex :type Integer) (bFromSweep :type Boolean) (SweepResult :type Hit%20Result%20Structure%20%28by%20ref%29))
  (Networking|SwitchHasAuthority
    (:Authority
      (CallFunction|Multicast)
      (Class|InterfaceBaseCharacter|ApplyDamage(Message) OtherActor (Variables|Default|Getdamage_id) self))))

(event Custom|multicast
  (Development|PrintString "Hello")
  (Audio|PlaySoundatLocation "/Game/StarterContent/Audio/Explosion01.Explosion01" (Transformation|GetActorLocation) "0, 0, 0" 1.0 1.0 0.0 0 0 0)
  (AddComponent|AddParticleSystemComponent false))

(event EventBeginPlay
  (Actor|Tick|AddTickPrerequisiteActor (Game|Player|GetPlayerPawn 0)))

(fn ConstructionScript)

(fn GetAttackTraceChannel
  (return "TraceTypeQuery1"))

(fn GetBasePower
  (return 1e+01))

(fn GetCharacterState
  (return "Walk_and_Jump"))

(fn GetCurrentVelocity
  (return "0, 0, 0"))

(fn GetDamageData
  (return (Variables|Default|Getdamage_data)))

(fn GetDurabilityLevel
  (return 0))

(fn GetIsonSprint
  (return false))

(fn GetLookDirection
  (return 0.0 0.0))

(fn GetLookRotation
  (return "0, 0, 0"))

(fn GetPrevSockLoc
  (return "0, 0, 0" "0, 0, 0"))

(fn GetTargetRotation
  (return "0, 0, 0"))

(fn GetWeapon
  (params (__key :type Name :default "None"))
  (return 0))