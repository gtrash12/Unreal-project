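; Player controller, marked discarded (폐기) in its name, that creates the local HUD, spawns a follow camera and runs target lock-on.
; Lock-on picks the unobstructed actor closest to camera forward by dot product, using visibility traces.
; Axis input switches targets by yaw side on a short cooldown, updating markers and state bars.
; It also relays damage through server-named events to the damaged actor's message.
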(event Custom|Server_ApplyDamage
  (params (damaged_actor :type Actor%20Object%20Reference) (damage_data :type Damage%20Data%20Structure) (damage_causor :type Actor%20Object%20Reference))
  (Class|BPIBaseCharacter|ApplyDamageBp(Message) damaged_actor damage_data damage_causor))

(event EventBeginPlay
  (bind _returnvalue (Game|Player|GetPlayerPawn 0))
  ;[1 1 1] Spawn and set Smooth Camera
  (Utilities|FlowControl|Sequence
    (:then_0
      (if (and (not (Networking|IsDedicatedServer)) (Pawn|IsLocalPlayerController))
        (bind _returnvalue_2 (UserInterface|CreateWidget "/Game/Blueprint/Widget_UI.Widget_UI_C"))
        (bind _output_get (Variables|Default|SetHUD_reference _returnvalue_2))
        (UserInterface|Viewport|AddtoViewport _output_get 0)))
    (:then_1
      (Utilities|FlowControl|Delay 2.0)
      (bind _returnvalue_3 (Game|SpawnActorfromClass "/Game/Blueprint/Camera_BP.Camera_BP_C" (Transformation|GetActorTransform _returnvalue) "Undefined" 0 0))
      (bind _asbp_base_character (Utilities|Casting|CastToBP_BaseCharacter _returnvalue))
      (Variables|/Game/Blueprint/Camera_BP.Camera_BP_C|SetTarget _returnvalue_3 _asbp_base_character)
      (Game|Player|SetViewTargetwithBlend (Game|GetPlayerController 0) _returnvalue_3 0.0 "VTBlend_Linear" 0.0 false)
      (Variables|Default|Setfollow_cam _returnvalue_3))))

(event EventTick
  (params (DeltaSeconds :type Float%20%28single-precision%29))
  (|CallParentFunction DeltaSeconds)
  (Variables|Default|Setlock_on_cooltime (- (Variables|Default|Getlock_on_cooltime) DeltaSeconds)))

(event EventCtoSApplyDamage
  (params (danaged_actor :type Actor%20Object%20Reference) (damage_data :type Damage%20Data%20Structure) (damage_causor :type Actor%20Object%20Reference))
  (CallFunction|ServerApplyDamage danaged_actor damage_data damage_causor))

(event EventReleaseLockon
  (bind _follow_cam (Variables|Default|Getfollow_cam))
  (bind _follow_cam_2 (Variables|Default|Getfollow_cam))
  (bind _follow_cam_3 (Variables|Default|Getfollow_cam))
  (Utilities|IsValid _follow_cam_2
    (:Is%20Valid
      (Variables|/Game/Blueprint/Camera_BP.Camera_BP_C|Setlock_on _follow_cam_2 true)
      (if (Variables|/Game/Blueprint/Camera_BP.Camera_BP_C|Getlock_on _follow_cam)
        (Variables|/Game/Blueprint/Camera_BP.Camera_BP_C|Setlock_on _follow_cam false)
        (Class|BPIAI|SetLockonMarker(Message) (Variables|/Game/Blueprint/Camera_BP.Camera_BP_C|Getlock_on_target (Variables|Default|Getfollow_cam)) false)
        (Pawn|SetControlRotation (Transformation|GetSocketRotation (Variables|/Game/Blueprint/Camera_BP.Camera_BP_C|GetCamera (Variables|Default|Getfollow_cam)) "None"))
        (else
          (bind _target (CallFunction|FindLockonTarget))
          (Utilities|IsValid _target
            (:Is%20Valid
              (Class|BPIAI|SetLockonMarker(Message) (Variables|/Game/Blueprint/Camera_BP.Camera_BP_C|Getlock_on_target (Variables|Default|Getfollow_cam)) false)
              (Class|BPIAI|SetStateBarVisibility(Message) _target true)
              (Class|BPIAI|SetLockonMarker(Message) _target true)
              (Variables|/Game/Blueprint/Camera_BP.Camera_BP_C|Setlock_on _follow_cam_3 true)
              (Variables|/Game/Blueprint/Camera_BP.Camera_BP_C|Setlock_on_target _follow_cam_3 _target))))))))

(event Input|ActionEvents|InputActionLockOn
  (params (Key :type Key%20Structure))
  (bind _follow_cam (Variables|Default|Getfollow_cam))
  (bind _follow_cam_2 (Variables|Default|Getfollow_cam))
  (:Pressed
    (Utilities|IsValid _follow_cam
      (:Is%20Valid
        (if (Variables|/Game/Blueprint/Camera_BP.Camera_BP_C|Getlock_on _follow_cam)
          (Variables|/Game/Blueprint/Camera_BP.Camera_BP_C|Setlock_on _follow_cam false)
          (Class|BPIAI|SetLockonMarker(Message) (Variables|/Game/Blueprint/Camera_BP.Camera_BP_C|Getlock_on_target (Variables|Default|Getfollow_cam)) false)
          (Pawn|SetControlRotation (Transformation|GetSocketRotation (Variables|/Game/Blueprint/Camera_BP.Camera_BP_C|GetCamera (Variables|Default|Getfollow_cam)) "None"))
          (else
            (bind _target (CallFunction|FindLockonTarget))
            (Utilities|IsValid _target
              (:Is%20Valid
                (Class|BPIAI|SetLockonMarker(Message) (Variables|/Game/Blueprint/Camera_BP.Camera_BP_C|Getlock_on_target (Variables|Default|Getfollow_cam)) false)
                (Class|BPIAI|SetStateBarVisibility(Message) _target true)
                (Class|BPIAI|SetLockonMarker(Message) _target true)
                (Variables|/Game/Blueprint/Camera_BP.Camera_BP_C|Setlock_on _follow_cam_2 true)
                (Variables|/Game/Blueprint/Camera_BP.Camera_BP_C|Setlock_on_target _follow_cam_2 _target)))))))))

(event Input|AxisEvents|InputAxisChangeLockOn
  (params (AxisValue :type Float%20%28single-precision%29))
  (bind _follow_cam (Variables|Default|Getfollow_cam))
  (if (< (Variables|Default|Getlock_on_cooltime) 0.0)
    (Utilities|IsValid _follow_cam
      (:Is%20Valid
        (if (Variables|/Game/Blueprint/Camera_BP.Camera_BP_C|Getlock_on _follow_cam)
          (bind _target (CallFunction|ChangeLockonTarget AxisValue))
          (Utilities|IsValid _target
            (:Is%20Valid
              (Class|BPIAI|SetLockonMarker(Message) (Variables|/Game/Blueprint/Camera_BP.Camera_BP_C|Getlock_on_target (Variables|Default|Getfollow_cam)) false)
              (Class|BPIAI|SetStateBarVisibility(Message) _target true)
              (Class|BPIAI|SetLockonMarker(Message) _target true)
              (Variables|/Game/Blueprint/Camera_BP.Camera_BP_C|Setlock_on_target (Variables|Default|Getfollow_cam) _target)
              (Variables|Default|Setlock_on_cooltime 0.2))))))))

(fn ConstructionScript)

(fn FindLockonTarget
  (bind _follow_cam (Variables|Default|Getfollow_cam))
  (bind _camera (Variables|/Game/Blueprint/Camera_BP.Camera_BP_C|GetCamera _follow_cam))
  (bind _returnvalue (Transformation|GetSocketLocation _camera "None"))
  (bind _outactors (Actor|GetAllActorsOfClass "/Game/Blueprint/bpbp.bpbp_C"))
  (for _array_element _outactors
    (bind _returnvalue_2 (Collision|LineTraceByChannel _returnvalue (Transformation|GetActorLocation _array_element) "TraceTypeQuery1" false _outactors "None"))
    (if (not _returnvalue_2)
      (if (> (Math|Vector|DotProduct (Math|Vector|Normalize (Math|Vector|GetForwardVector (Math|Rotator|FindLookatRotation _returnvalue (Transformation|GetActorLocation _array_element)))) (Math|Vector|Normalize (Math|Vector|GetForwardVector (Transformation|GetSocketRotation _camera "None")))) (LocalVariables|Getmin_angle))
        (LocalVariables|Setmin_angle (Math|Vector|DotProduct (Math|Vector|Normalize (Math|Vector|GetForwardVector (Math|Rotator|FindLookatRotation _returnvalue (Transformation|GetActorLocation _array_element)))) (Math|Vector|Normalize (Math|Vector|GetForwardVector (Transformation|GetSocketRotation _camera "None")))))
        (LocalVariables|Setlock_on_target _array_element)
        (LocalVariables|Setmin_distance (Math|Vector|Distance(Vector) _returnvalue (Transformation|GetActorLocation _array_element)))
        (Development|PrintString (Utilities|GetDisplayName _array_element)))))
  (return (LocalVariables|Getlock_on_target)))

(fn ChangeLockonTarget
  (params (direction :type Float%20%28single-precision%29))
  (bind _follow_cam (Variables|Default|Getfollow_cam))
  (bind _camera (Variables|/Game/Blueprint/Camera_BP.Camera_BP_C|GetCamera _follow_cam))
  (LocalVariables|Setsocket_location (Transformation|GetSocketLocation _camera "None"))
  (LocalVariables|Setsocket_rotation (Transformation|GetSocketRotation _camera "None"))
  (LocalVariables|Settarget_foward_vector (Math|Vector|GetForwardVector (Math|Rotator|FindLookatRotation (LocalVariables|Getsocket_location) (Transformation|GetActorLocation (Variables|/Game/Blueprint/Camera_BP.Camera_BP_C|Getlock_on_target (Variables|Default|Getfollow_cam))))))
  (bind _outactors (Actor|GetAllActorsOfClass "/Game/Blueprint/bpbp.bpbp_C"))
  (for _array_element _outactors
    (if (!= (Variables|/Game/Blueprint/Camera_BP.Camera_BP_C|Getlock_on_target (Variables|Default|Getfollow_cam)) _array_element)
      (bind _returnvalue (Collision|LineTraceByChannel (LocalVariables|Getsocket_location) (Transformation|GetActorLocation _array_element) "TraceTypeQuery1" false _outactors "None"))
      (if (not _returnvalue)
        (if (> (Math|Vector|DotProduct (Math|Vector|Normalize (Math|Vector|GetForwardVector (Math|Rotator|FindLookatRotation (LocalVariables|Getsocket_location) (Transformation|GetActorLocation _array_element)))) (Math|Vector|Normalize (Math|Vector|GetForwardVector (LocalVariables|Getsocket_rotation)))) 0.6)
          (if (> (* (.Yaw (Math|Vector|GetYawPitchfromVector (Math|Vector|UnrotateVector (- (Math|Vector|GetForwardVector (Math|Rotator|FindLookatRotation (LocalVariables|Getsocket_location) (Transformation|GetActorLocation _array_element))) (Math|Vector|GetForwardVector (LocalVariables|Getsocket_rotation))) (LocalVariables|Getsocket_rotation)))) direction) 1e+01)
            (if (> (Math|Vector|DotProduct (Math|Vector|Normalize (Math|Vector|GetForwardVector (Math|Rotator|FindLookatRotation (LocalVariables|Getsocket_location) (Transformation|GetActorLocation _array_element)))) (Math|Vector|Normalize (Math|Vector|GetForwardVector (LocalVariables|Getsocket_rotation)))) (LocalVariables|Getmin_angle))
              (LocalVariables|Setmin_angle (Math|Vector|DotProduct (Math|Vector|Normalize (Math|Vector|GetForwardVector (Math|Rotator|FindLookatRotation (LocalVariables|Getsocket_location) (Transformation|GetActorLocation _array_element)))) (Math|Vector|Normalize (Math|Vector|GetForwardVector (LocalVariables|Getsocket_rotation)))))
              (LocalVariables|Setlock_on_target _array_element)))))))
  (return (LocalVariables|Getlock_on_target)))

(fn GetLockonTarget
  (return (Variables|/Game/Blueprint/Camera_BP.Camera_BP_C|Getlock_on_target (Variables|Default|Getfollow_cam))))

(fn IsLockonTarget
  (params (actor :type Actor%20Object%20Reference))
  (return (== actor (Variables|/Game/Blueprint/Camera_BP.Camera_BP_C|Getlock_on_target (Variables|Default|Getfollow_cam)))))