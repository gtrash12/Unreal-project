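; BlockingWall is an interactable obstacle that teleports the player when they interact while facing the required direction.
; A dot product between view direction and the wall's rotated forward vector gates both the HUD interact prompt and the interaction.
; Interaction snaps the player to the wall's rotation with a pitch offset, then moves them a short fixed distance along that forward vector without sweeping.
; A fast-roll montage call exists but is disconnected.
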(event EventInteraction
  (params (causor :type Actor%20Object%20Reference))
  (bind _returnvalue (Transformation|GetActorRotation))
  (bind _returnvalue_2 (+ (.pitch _returnvalue) -9e+01))
  (bind _returnvalue_3 (Math|Rotator|MakeRotator (.roll _returnvalue) _returnvalue_2 (.yaw _returnvalue)))
  (bind ___look_rotation (Class|InterfaceBaseCharacter|GetLookRotation(Message) causor))
  (if (> (Math|Vector|DotProduct (Math|Vector|RotateVector (Transformation|GetActorForwardVector) "-90.000000, 0, 0") (Math|Vector|GetForwardVector ___look_rotation)) 0.5)
    (bind _asbp_player_character_cpp (Utilities|Casting|CastToBP_PlayerCharacter_cpp causor))
    (Transformation|SetActorRotation _asbp_player_character_cpp _returnvalue_3)
    (Transformation|SetActorLocation _asbp_player_character_cpp (+ (Transformation|GetActorLocation _asbp_player_character_cpp) (* (Math|Vector|GetForwardVector _returnvalue_3) 7e+01)) false true)))

(event EventPopInteractionInfo
  (params (causor :type Actor%20Object%20Reference))
  (if (> (Math|Vector|DotProduct (Math|Vector|RotateVector (Transformation|GetActorForwardVector) "-90.000000, 0, 0") (Math|Vector|GetForwardVector (Pawn|GetControlRotation (Game|GetPlayerController 0) :!class /Script/Engine.Controller))) 0.5)
    (bind _ascontroller_player_character_cpp (Utilities|Casting|CastToController_PlayerCharacter_cpp (Game|GetPlayerController 0)))
    (Utilities|IsValid (Variables|/Game/Blueprint/controller/Controller_PlayerCharacter_cpp.Controller_PlayerCharacter_cpp_C|GetHUD_reference _ascontroller_player_character_cpp)
      (:Is%20Valid
        (Widget|SetVisibility (Variables|/Game/Blueprint/Widget/Widget_UI.Widget_UI_C|GetInteractBox (Variables|/Game/Blueprint/controller/Controller_PlayerCharacter_cpp.Controller_PlayerCharacter_cpp_C|GetHUD_reference _ascontroller_player_character_cpp)) "Visible")))))

(event EventRemoveInteractionInfo
  (params (causor :type Actor%20Object%20Reference))
  (bind _ascontroller_player_character_cpp (Utilities|Casting|CastToController_PlayerCharacter_cpp (Game|GetPlayerController 0)))
  (Utilities|IsValid (Variables|/Game/Blueprint/controller/Controller_PlayerCharacter_cpp.Controller_PlayerCharacter_cpp_C|GetHUD_reference _ascontroller_player_character_cpp)
    (:Is%20Valid
      (Widget|SetVisibility (Variables|/Game/Blueprint/Widget/Widget_UI.Widget_UI_C|GetInteractBox (Variables|/Game/Blueprint/controller/Controller_PlayerCharacter_cpp.Controller_PlayerCharacter_cpp_C|GetHUD_reference _ascontroller_player_character_cpp)) "Hidden"))))

(fn ConstructionScript)