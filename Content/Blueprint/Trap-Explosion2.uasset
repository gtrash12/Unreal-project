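; Explosion trap actor that knocks characters away when they overlap its cylinder.
; On the server, any overlap multicasts the explosion sound and particle effect, then a BP_BaseCharacter has its montage stopped.
; Unless a state check blocks it, the character is launched radially outward plus upward, then gets a multicast state change about two frames later.
; OffOption then switches the cylinder to physics-only collision, disabling further overlaps.
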(event OnComponentBeginOverlap(Cylinder)
  (params (OverlappedComponent :type Primitive%20Component%20Object%20Reference) (OtherActor :type Actor%20Object%20Reference) (OtherComp :type Primitive%20Component%20Object%20Reference) (OtherBodyIndex :type Integer) (bFromSweep :type Boolean) (SweepResult :type Hit%20Result%20Structure%20%28by%20ref%29))
  (Networking|SwitchHasAuthority
    (:Authority
      (CallFunction|Multicast)
      (bind _asbp_base_character (Utilities|Casting|CastToBP_BaseCharacter OtherActor))
      (Class|AnimInstance|MontageStopGroupbyName (Variables|/Game/Blueprint/BP_BaseCharacter.BP_BaseCharacter_C|GetMainAnimInstance _asbp_base_character) 0.0 "DefaultGroup")
      (bind _chk (Default|StateChk _asbp_base_character "NewEnumerator4"))
      (if (not _chk)
        (Character|LaunchCharacter _asbp_base_character (+ (* (Math|Vector|Normalize (- (Transformation|GetActorLocation _asbp_base_character) (Transformation|GetActorLocation self))) (Variables|Default|GetNuckbackVelocity)) (* (Math|Vector|VectorUp) (Variables|Default|GetUpVelocity))) true true)
        (Utilities|FlowControl|Delay (* (Utilities|Time|GetWorldDeltaSeconds) 2.0))
        (Default|SetStateMulticast _asbp_base_character "NewEnumerator2")
        (if (Variables|Default|GetOffOption)
          (Collision|SetCollisionEnabled (Variables|Default|GetCylinder) "PhysicsOnly"))))))

(event Custom|multicast
  (Audio|PlaySoundatLocation "/Game/StarterContent/Audio/Explosion01.Explosion01" (Transformation|GetActorLocation) "0, 0, 0" 1.0 1.0 0.0 0 0 0)
  (AddComponent|AddParticleSystemComponent false))

(event EventBeginPlay
  (Actor|Tick|AddTickPrerequisiteActor (Game|Player|GetPlayerPawn 0)))

(fn ConstructionScript)