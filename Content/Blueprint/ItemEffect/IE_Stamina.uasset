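; IE_Stamina is an item effect that restores the player's stamina and current maximum stamina.
; When applied, it casts a valid Causor to BP_PlayerCharacter_cpp and adds Value to both Stamina and CurMaxStamina, with no clamp in this graph.
; DescribeItemEffect returns Korean text stating that the item restores maximum stamina by that Value.
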(event EventApplyItemEffect
  (params (causor :type Character%20Object%20Reference) (__inven_index :type Integer))
  (bind _value (Variables|Default|Getvalue))
  (Utilities|IsValid causor
    (:Is%20Valid
      (bind _asbp_player_character_cpp (Utilities|Casting|CastToBP_PlayerCharacter_cpp causor))
      (Variables|/Script/CyperArena.BaseCharacter|Setstamina _asbp_player_character_cpp (+ (Variables|/Script/CyperArena.BaseCharacter|Getstamina _asbp_player_character_cpp) _value))
      (Variables|/Script/CyperArena.BaseCharacter|Setcur_max_stamina _asbp_player_character_cpp (+ (Variables|/Script/CyperArena.BaseCharacter|Getcur_max_stamina _asbp_player_character_cpp) _value)))))

(fn DescribeItemEffect
  (return (Utilities|Text|FormatText "스테미너 최대치를 {value} 회복합니다." (Variables|Default|Getvalue))))