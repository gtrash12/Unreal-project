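; IE_DecreaseCount is an item effect that consumes one unit of the item in a given inventory slot.
; On ApplyItemEffect it casts the causer's controller to the player controller and, if the slot exists in InventoryList, re-adds it with the count lowered by one.
; If that slot maps to a quickslot through ReverseQuickslotList, it refreshes that quickslot; entries are not removed or clamped at zero.
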(event EventApplyItemEffect
  (params (causor :type Character%20Object%20Reference) (__inven_index :type Integer))
  (bind _ascontroller_player_character_cpp_2 (Utilities|Casting|CastToController_PlayerCharacter_cpp_2 (Pawn|GetController causor)))
  (if (.ReturnValue (Utilities|Map|Find (Variables|/Script/CyperArena.Controller_Player|Getinventory_list _ascontroller_player_character_cpp_2) __inven_index))
    (Utilities|Map|Add (Variables|/Script/CyperArena.Controller_Player|Getinventory_list _ascontroller_player_character_cpp_2) __inven_index (Utilities|Struct|MakeInventoryData (.item_id (.Value (Utilities|Map|Find (Variables|/Script/CyperArena.Controller_Player|Getinventory_list _ascontroller_player_character_cpp_2) __inven_index))) (- (.count (.Value (Utilities|Map|Find (Variables|/Script/CyperArena.Controller_Player|Getinventory_list _ascontroller_player_character_cpp_2) __inven_index))) 1)))
    (if (.ReturnValue (Utilities|Map|Find (Variables|/Script/CyperArena.Controller_Player|Getreverse_quickslot_list _ascontroller_player_character_cpp_2) __inven_index))
      (Class|ControllerPlayer|RefreshQuickSlot _ascontroller_player_character_cpp_2 (.Value (Utilities|Map|Find (Variables|/Script/CyperArena.Controller_Player|Getreverse_quickslot_list _ascontroller_player_character_cpp_2) __inven_index))))))