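; Item effect that raises the player character's action speed while it is registered.
; On registration it adds Value to the BP_PlayerCharacter_cpp ActionSpeed, and on removal it subtracts the same amount.
; Causors that are not that character class are ignored.
; DescribeItemEffect returns Korean text showing Value as a percentage bonus to all action speed.
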(event EventOnRegistration
  (params (causor :type Character%20Object%20Reference) (__inven_index :type Integer))
  (bind _asbp_player_character_cpp (Utilities|Casting|CastToBP_PlayerCharacter_cpp causor))
  (Variables|/Game/Blueprint/Character/BP_PlayerCharacter_cpp.BP_PlayerCharacter_cpp_C|Setaction_speed _asbp_player_character_cpp (+ (Variables|/Game/Blueprint/Character/BP_PlayerCharacter_cpp.BP_PlayerCharacter_cpp_C|Getaction_speed _asbp_player_character_cpp) (Variables|Default|Getvalue))))

(event EventOnRemoveRegistration
  (params (causor :type Character%20Object%20Reference) (__inven_index :type Integer))
  (bind _asbp_player_character_cpp (Utilities|Casting|CastToBP_PlayerCharacter_cpp causor))
  (Variables|/Game/Blueprint/Character/BP_PlayerCharacter_cpp.BP_PlayerCharacter_cpp_C|Setaction_speed _asbp_player_character_cpp (+ (Variables|/Game/Blueprint/Character/BP_PlayerCharacter_cpp.BP_PlayerCharacter_cpp_C|Getaction_speed _asbp_player_character_cpp) (* -1 (Variables|Default|Getvalue)))))

(fn DescribeItemEffect
  (return (Utilities|Text|FormatText "모든 액션 속도 + {value}%" (* 100 (Variables|Default|Getvalue)))))