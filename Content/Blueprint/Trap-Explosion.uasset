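; Explosion trap that knocks a player character back when something overlaps its collision component.
; The overlap spawns a particle effect, then casts the other actor to Player_Character_BP.
; The launch overrides current velocity, combining the unnormalized trap-to-player offset scaled by a knockback value with an upward boost.
; After a brief delay, it sets the player's state through a multicast call.
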(event OnComponentBeginOverlap(CollisionComponent)
  (params (OverlappedComponent :type Primitive%20Component%20Object%20Reference) (OtherActor :type Actor%20Object%20Reference) (OtherComp :type Primitive%20Component%20Object%20Reference) (OtherBodyIndex :type Integer) (bFromSweep :type Boolean) (SweepResult :type Hit%20Result%20Structure%20%28by%20ref%29))
  (AddComponent|AddParticleSystemComponent false)
  (Networking|SwitchHasAuthority
    (:Authority
      _)
    (:Remote
      _))
  (bind _asplayer_character_bp (Utilities|Casting|CastToPlayer_Character_BP OtherActor))
  (Character|LaunchCharacter _asplayer_character_bp (+ (* (- (Transformation|GetActorLocation _asplayer_character_bp) (Transformation|GetActorLocation self)) (Variables|Default|GetNuckbackVelocity)) (* (Math|Vector|VectorUp) (Variables|Default|GetUpVelocity))) true true)
  (Utilities|FlowControl|Delay 0.02)
  (Default|SetStateMulticast _asplayer_character_bp "NewEnumerator2"))

(event OnComponentSleep(CollisionComponent)
  (params (SleepingComponent :type Primitive%20Component%20Object%20Reference) (BoneName :type Name :default "None")))

(fn ConstructionScript)