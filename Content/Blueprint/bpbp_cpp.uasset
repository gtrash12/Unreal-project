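; Enemy character Blueprint on a parent class, with an overhead health bar, lock-on marker and functions for combat AI.
; Damage retargets the enemy controller to the causer and updates the bar; death triggers an impulsed ragdoll, releases player lock-on and destroys the actor after a delay.
; BTGraph handles montage attacks turned toward the target, sprint speed and interpolated, clamped look pitch/yaw.
; Tick disables orient-to-movement during knockback.
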(event EventBeginPlay
  (|CallParentFunction)
  (bind _aswidget_enemy_health_bar (Utilities|Casting|CastToWidget_EnemyHealthBar (UserInterface|GetWidget (Variables|Default|GetStatebar))))
  (Default|Init _aswidget_enemy_health_bar self)
  (Variables|/Script/Engine.CharacterMovementComponent|SetMaxWalkSpeed (Variables|Character|GetCharacterMovement) (Variables|Default|Getwalk_speed)))

(event Collision|EventActorBeginOverlap
  (params (OtherActor :type Actor%20Object%20Reference)))

(event EventTick
  (params (DeltaSeconds :type Float%20%28single-precision%29))
  (|CallParentFunction DeltaSeconds)
  (if (> (Variables|Default|Getknock_back_speed) 0.0)
    (Variables|/Script/Engine.CharacterMovementComponent|SetbOrientRotationToMovement (Variables|Character|GetCharacterMovement) false)
    (else
      (Variables|/Script/Engine.CharacterMovementComponent|SetbOrientRotationToMovement (Variables|Character|GetCharacterMovement) true))))

(event EventApplyDamageMulticastExec
  (params (target_damage_data :type Damage%20Data%20Structure) (damage_causor :type Actor%20Object%20Reference))
  (bind _returnvalue (Game|GetPlayerController 0))
  (bind _hp (Variables|Default|Gethp))
  (|CallParentFunction target_damage_data damage_causor)
  (bind _output_get (Variables|Default|Settarget_actor damage_causor))
  (bind _ascontroller_enemy (Utilities|Casting|CastToController_Enemy (Pawn|GetController))
    (:then
      (Default|TargetChange _ascontroller_enemy _output_get))
    (:CastFailed
      _))
  (bind _aswidget_enemy_health_bar (Utilities|Casting|CastToWidget_EnemyHealthBar (UserInterface|GetWidget (Variables|Default|GetStatebar))))
  (Default|Update _aswidget_enemy_health_bar (/ _hp (Variables|Default|Getmax_hp)))
  (if (<= _hp 0.0)
    (CallFunction|SetStateBarVisibility false)
    (Utilities|FlowControl|Delay 0.2)
    (Class|BaseCharacter|SetCharacterState "Ragdoll")
    (Class|SkeletalMeshComponent|AddImpulsetoAllBodiesBelow (Variables|Character|GetMesh) (+ (* (Transformation|GetVelocity) "10.000000,10.000000,3.000000") "0,0.000000,100.000000") "pelvis" false true)
    (bind _result (Class|InterfacePlayerController|IsLockonTarget(Message) _returnvalue self))
    (if _result
      (Class|InterfacePlayerController|ReleaseLockON(Message) _returnvalue))
    (Utilities|FlowControl|Sequence
      (:then_0
        (Collision|SetCollisionEnabled (Variables|Default|GetCapsuleComponent) "NoCollision")
        (Collision|SetCollisionEnabled (Variables|Character|GetMesh) "PhysicsOnly")
        (Components|DestroyComponent (Variables|Default|GetLockOnMarker))
        (Components|DestroyComponent (Variables|Default|GetStatebar)))
      (:then_1
        (Utilities|FlowControl|Delay 3.0)
        (Actor|DestroyActor)))
    (else
      (CallFunction|SetStateBarVisibility true))))

(event EventSetLockonMarker
  (params (onoff :type Boolean))
  (bind _lockonmarker (Variables|Default|GetLockOnMarker))
  (Utilities|IsValid _lockonmarker
    (:Is%20Valid
      (Rendering|SetVisibility _lockonmarker onoff false))))

(event EventSetStateBarVisibility
  (params (onoff :type Boolean))
  (bind _statebar (Variables|Default|GetStatebar))
  (Utilities|IsValid _statebar
    (:Is%20Valid
      (Rendering|SetVisibility _statebar onoff false)
      (Widget|SetVisibility (UserInterface|GetWidget _statebar) "Visible"))))

(event Custom|AttackMulticast
  (params (last_movement_input :type Vector) (animation :type Anim%20Montage%20Object%20Reference))
  (Animation|PlayAnimMontage animation 1.0 "None")
  (Class|BaseCharacter|RotateActorwithinTime (Math|Rotator|MakeRotfromX last_movement_input) 0.4))

(event Custom|SprintMulticast
  (params (IsSprint :type Boolean))
  (bind _output_get (Variables|Default|Setis_on_sprint IsSprint))
  (Variables|/Script/Engine.CharacterMovementComponent|SetMaxWalkSpeed (Variables|Character|GetCharacterMovement) (Math|Float|SelectFloat (Variables|Default|Getsprint_speed) (Variables|Default|Getwalk_speed) _output_get)))

(event EventSetLookRotation
  (bind _target_actor (Variables|Default|Gettarget_actor)
    (:then
      (Variables|Default|Setlook_location (Transformation|GetActorLocation _target_actor)))
    (:else
      _))
  (Variables|Default|Setlook_pitch (Math|Float|ClampAngle (.Pitch (Math|Rotator|BreakRotator (Math|Interpolation|RInterpTo (Math|Rotator|MakeRotator 0.0 (Variables|Default|Getlook_pitch) (Variables|Default|Getlook_yaw)) (Math|Rotator|Delta(Rotator) (Math|Rotator|FindLookatRotation (Transformation|GetActorLocation) (Variables|Default|Getlook_location)) (Transformation|GetActorRotation)) (Utilities|Time|GetWorldDeltaSeconds) 3.0))) -9e+01 9e+01))
  (Variables|Default|Setlook_yaw (Math|Float|ClampAngle (.Yaw (Math|Rotator|BreakRotator (Math|Interpolation|RInterpTo (Math|Rotator|MakeRotator 0.0 (Variables|Default|Getlook_pitch) (Variables|Default|Getlook_yaw)) (Math|Rotator|Delta(Rotator) (Math|Rotator|FindLookatRotation (Transformation|GetActorLocation) (Variables|Default|Getlook_location)) (Transformation|GetActorRotation)) (Utilities|Time|GetWorldDeltaSeconds) 3.0))) -9e+01 9e+01)))

(event EventSetSprint
  (params (is_sprint :type Boolean))
  (CallFunction|SprintMulticast is_sprint))

(event EventAttack
  (if (not (Class|AnimInstance|IsAnyMontagePlaying (Variables|Default|Getmain_anim_instance)))
    (switch Utilities|FlowControl|Switch|SwitchonECharacterState (Variables|Default|Getcharacter_state)
      (:Walk_and_Jump
        (CallFunction|AttackMulticast (Math|Vector|GetForwardVector (Math|Rotator|FindLookatRotation (Transformation|GetActorLocation) (Transformation|GetActorLocation (Variables|Default|Gettarget_actor)))) (Variables|Default|Getnext_attack_montage))))))

(event EventSetLookLocation
  (params (target_location :type Vector :default "0, 0, 0"))
  (Variables|Default|Setlook_location target_location))

(event EventSetTarget
  (params (target :type Actor%20Object%20Reference))
  (Variables|Default|Settarget_actor target))

(fn ConstructionScript
  (|CallParentFunction))

(fn GetAttackTraceChannelBp
  (return "TraceTypeQuery5"))

(fn GetAttackTraceChannel
  (return "TraceTypeQuery5"))

(fn GetTarget
  (return (Variables|Default|Gettarget_actor)))