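; Enemy character Blueprint with a widget health bar, lock-on marker and events for AI-driven combat and movement.
; BTGraph events set target and sprint speed, play attack montages turned toward the target, and interpolate clamped look pitch/yaw.
; Damage extends the parent's multicast handler, retargeting the enemy controller to the attacker and updating the health bar.
; At zero HP it ragdolls with a velocity-based impulse, releases player lock-on, then destroys itself after a delay.
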(event EventBeginPlay
  (|CallParentFunction)
  (bind _aswidget_enemy_health_bar (Utilities|Casting|CastToWidget_EnemyHealthBar (UserInterface|GetWidget (Variables|Default|GetStatebar))))
  (Default|Init _aswidget_enemy_health_bar self)
  (Variables|/Script/Engine.CharacterMovementComponent|SetMaxWalkSpeed (Variables|Character|GetCharacterMovement) (Variables|Default|GetWalkSpeed)))

(event Collision|EventActorBeginOverlap
  (params (OtherActor :type Actor%20Object%20Reference)))

(event EventTick
  (params (DeltaSeconds :type Float%20%28single-precision%29))
  (|CallParentFunction DeltaSeconds))

(event EventSetLockonMarker
  (params (onoff :type Boolean))
  (bind _lockonmarker (Variables|Default|GetLockOnMarker))
  (Utilities|IsValid _lockonmarker
    (:Is%20Valid
      (Rendering|SetVisibility _lockonmarker onoff false))))

(event EventSetStateBarVisibility
  (params (onoff :type Boolean))
  (bind _statebar (Variables|Default|GetStatebar))
  (Utilities|IsValid _statebar
    (:Is%20Valid
      (Rendering|SetVisibility _statebar onoff false)
      (Widget|SetVisibility (UserInterface|GetWidget _statebar) "Visible"))))

(event EventMulticastApplyDamage
  (params (damage_data :type Damage%20Data%20Structure) (damage_causor :type Actor%20Object%20Reference))
  (bind _returnvalue (Game|GetPlayerController 0))
  (bind _hp (Variables|Default|Gethp))
  (|CallParentFunction damage_data damage_causor)
  (bind _output_get (Variables|Default|Settarget_actor damage_causor))
  (bind _ascontroller_enemy (Utilities|Casting|CastToController_Enemy (Pawn|GetController))
    (:then
      (Default|TargetChange _ascontroller_enemy _output_get))
    (:CastFailed
      _))
  (bind _aswidget_enemy_health_bar (Utilities|Casting|CastToWidget_EnemyHealthBar (UserInterface|GetWidget (Variables|Default|GetStatebar))))
  (Default|Update _aswidget_enemy_health_bar (/ _hp (Variables|Default|Getmax_hp)))
  (if (<= _hp 0.0)
    (CallFunction|SetStateBarVisibility false)
    (Utilities|FlowControl|Delay 0.2)
    (CallFunction|SetState "Ragdoll")
    (Class|SkeletalMeshComponent|AddImpulsetoAllBodiesBelow (Variables|Character|GetMesh) (+ (* (Variables|Default|Getcurrent_velocity) "10.000000,10.000000,3.000000") "0,0.000000,100.000000") "pelvis" false true)
    (bind _result (Class|InterfacePlayerController|IsLockonTarget(Message) _returnvalue self))
    (if _result
      (Class|InterfacePlayerController|ReleaseLockON(Message) _returnvalue))
    (Utilities|FlowControl|Sequence
      (:then_0
        (Collision|SetCollisionEnabled (Variables|Default|GetCapsuleComponent) "NoCollision")
        (Collision|SetCollisionEnabled (Variables|Character|GetMesh) "PhysicsOnly")
        (Components|DestroyComponent (Variables|Default|GetLockOnMarker))
        (Components|DestroyComponent (Variables|Default|GetStatebar)))
      (:then_1
        (Utilities|FlowControl|Delay 3.0)
        (Actor|DestroyActor)))
    (else
      (CallFunction|SetStateBarVisibility true))))

(event Custom|AttackMulticast
  (params (last_movement_input :type Vector) (animation :type Anim%20Montage%20Object%20Reference))
  (Animation|PlayAnimMontage animation 1.0 "None")
  (CallFunction|RotateLastInput 0.7 last_movement_input))

(event Custom|SprintMulticast
  (params (IsSprint :type Boolean))
  (bind _output_get (Variables|Default|SetOnSprint IsSprint))
  (Variables|/Script/Engine.CharacterMovementComponent|SetMaxWalkSpeed (Variables|Character|GetCharacterMovement) (Math|Float|SelectFloat (Variables|Default|GetSprintSpeed) (Variables|Default|GetWalkSpeed) _output_get)))

(event EventSetLookRotation
  (bind _target_actor (Variables|Default|Gettarget_actor)
    (:then
      (Variables|Default|Setlook_location (Transformation|GetActorLocation _target_actor)))
    (:else
      _))
  (Variables|Default|Setlook_pitch (Math|Float|ClampAngle (.Pitch (Math|Rotator|BreakRotator (Math|Interpolation|RInterpTo (Math|Rotator|MakeRotator 0.0 (Variables|Default|Getlook_pitch) (Variables|Default|Getlook_yaw)) (Math|Rotator|Delta(Rotator) (Math|Rotator|FindLookatRotation (Transformation|GetActorLocation) (Variables|Default|Getlook_location)) (Transformation|GetActorRotation)) (Utilities|Time|GetWorldDeltaSeconds) 3.0))) -9e+01 9e+01))
  (Variables|Default|Setlook_yaw (Math|Float|ClampAngle (.Yaw (Math|Rotator|BreakRotator (Math|Interpolation|RInterpTo (Math|Rotator|MakeRotator 0.0 (Variables|Default|Getlook_pitch) (Variables|Default|Getlook_yaw)) (Math|Rotator|Delta(Rotator) (Math|Rotator|FindLookatRotation (Transformation|GetActorLocation) (Variables|Default|Getlook_location)) (Transformation|GetActorRotation)) (Utilities|Time|GetWorldDeltaSeconds) 3.0))) -9e+01 9e+01)))

(event EventRotateActorTimeline
  (params (__target_rotation :type Rotator :default "0, 0, 0") (__time :type Float%20%28single-precision%29))
  (bind _rotatelastinputtimeline (Variables|Default|GetRotateLastInputTimeline))
  (bind _output_get (Variables|Default|Settmp_rotation (Transformation|GetActorRotation)))
  (Audio|Components|Audio|Stop _rotatelastinputtimeline)
  (Components|Timeline|SetPlayRate _rotatelastinputtimeline (/ 1.0 __time))
  (bind _새_트랙_0 (Timeline|타임라인_1 PlayFromStart)
    (:Update
      (Transformation|SetActorRotation (Math|Interpolation|Ease "ExpoOut" _새_트랙_0 _output_get __target_rotation true) true))))

(event EventSetSprint
  (params (is_sprint :type Boolean))
  (CallFunction|SprintMulticast is_sprint))

(event EventAttack
  (if (not (Class|AnimInstance|IsAnyMontagePlaying (Variables|Default|GetMainAnimInstance)))
    (switch Utilities|FlowControl|Switch|SwitchonECharacterState (Variables|Default|GetState)
      (:Walk_and_Jump
        (CallFunction|AttackMulticast (Math|Vector|GetForwardVector (Math|Rotator|FindLookatRotation (Transformation|GetActorLocation) (Transformation|GetActorLocation (Variables|Default|Gettarget_actor)))) (Variables|Default|GetNextAttackMontage))))))

(event EventSetLookLocation
  (params (target_location :type Vector :default "0, 0, 0"))
  (Variables|Default|Setlook_location target_location))

(event EventSetTarget
  (params (target :type Actor%20Object%20Reference))
  (Variables|Default|Settarget_actor target))

(fn ConstructionScript
  (|CallParentFunction))

(fn GetAttackTraceChannelBp
  (return "TraceTypeQuery5"))

(fn GetAttackTraceChannel
  (return "TraceTypeQuery5"))

(fn GetTarget
  (return (Variables|Default|Gettarget_actor)))