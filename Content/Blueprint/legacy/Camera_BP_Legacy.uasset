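; Legacy camera actor that smoothly follows a Target's camera boom and control rotation.
; Each tick it interpolates its location toward the point from the Target's GetCameraBoom and its rotation toward the control rotation, both at the same fixed speed.
; On BeginPlay it adds the Target as a tick prerequisite, so the camera updates after the Target has ticked.
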(event EventBeginPlay
  (Actor|Tick|AddTickPrerequisiteActor (Variables|Default|GetTarget)))

(event EventTick
  (params (DeltaSeconds :type Float%20%28single-precision%29))
  (bind _target (Variables|Default|GetTarget))
  (bind _newparam (Default|GetCameraBoom _target))
  (Transformation|SetActorLocation (Math|Interpolation|VInterpTo (Transformation|GetActorLocation) _newparam DeltaSeconds 1e+01) false false)
  (Transformation|SetActorRotation (Math|Interpolation|RInterpTo (Transformation|GetActorRotation) (Pawn|GetControlRotation _target :!class /Script/Engine.Pawn) DeltaSeconds 1e+01)))

(fn ConstructionScript)