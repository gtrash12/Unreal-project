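; AN_Footstep is an animation notify that plays a footstep sound on the animated skeletal mesh.
; After validating the mesh and sound, it spawns the sound attached at a configurable attach point and volume, stopping it if the attached component is destroyed.
; It then passes the footstep type to the spawned audio component as the integer "FootstepType" parameter, so the sound asset can vary by type.
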(fn ReceivedNotify
  (params (MeshComp :type Skeletal%20Mesh%20Component%20Object%20Reference) (Animation :type Anim%20Sequence%20Base%20Object%20Reference))
  (Utilities|IsValid MeshComp
    (:Is%20Valid
      (bind _sound (Variables|Default|Getsound)
        (:then
          (bind _returnvalue (Audio|SpawnSoundAttached _sound MeshComp (Variables|Default|Getattach_point) "0, 0, 0" "0, 0, 0" "KeepRelativeOffset" true (Variables|Default|Getvolume) 1.0 0.0 0 0))
          (Utilities|IsValid _returnvalue
            (:Is%20Valid
              (Effects|Components|ParticleSystem|SetIntParameter _returnvalue "FootstepType" (Math|Conversions|ToInteger(Byte) (Variables|Default|Getfootstep_type)))
              (return false))))
        (:else)))))