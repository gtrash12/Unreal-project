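; Base multiplayer character with a state machine for locomotion, attack, airborne, ragdoll and get-up, plus dodge speed, look smoothing and sword damage.
; An airborne capsule hit triggers a multicast ragdoll.
; The controlling machine tracks the pelvis, sending it to the server when remote, while others drag the pelvis by physics handle and interpolate the actor, snapped to ground by trace.
; Get-up restores movement replication, saves a pose snapshot and plays a front or back montage.
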(event OnComponentHit(CapsuleComponent)
  (params (HitComponent :type Primitive%20Component%20Object%20Reference) (OtherActor :type Actor%20Object%20Reference) (OtherComp :type Primitive%20Component%20Object%20Reference) (NormalImpulse :type Vector :default "0, 0, 0") (Hit :type Hit%20Result%20Structure%20%28by%20ref%29))
  ;[1 1 1] Airbone collision check
  (Networking|SwitchHasAuthority
    (:Authority
      (if (Pawn|IsPlayerControlled)
        (switch Utilities|FlowControl|Switch|SwitchonCharacterState (Variables|캐릭터상태관련|GetState) :!label _label
          (:NewEnumerator2
            (CallFunction|RagdollSetonServer)))))
    (:Remote
      (if (Pawn|IsLocallyControlled)
        (goto _label)))))

(event OnComponentBeginOverlap(SK_Sword)
  (params (OverlappedComponent :type Primitive%20Component%20Object%20Reference) (OtherActor :type Actor%20Object%20Reference) (OtherComp :type Primitive%20Component%20Object%20Reference) (OtherBodyIndex :type Integer) (bFromSweep :type Boolean) (SweepResult :type Hit%20Result%20Structure%20%28by%20ref%29))
  (bind _damage_data (Variables|공격관련|Getdamage_data))
  (if (!= (Components|GetOwner OtherActor) (Components|GetOwner))
    (Development|PrintString (.name _damage_data))
    (Game|Damage|ApplyDamage OtherActor (.base_damage_percent _damage_data) 0 0 "/Script/Engine.DamageType")))

(event Custom|RagdollSetonServer
  ;[1 1 1] 래그돌 서버 세팅
  (Variables|래그돌관련|SetRagdollServerLocation (Transformation|GetSocketLocation (Variables|Character|GetMesh) "pelvis"))
  (CallFunction|RagdollSetMult))

(event Custom|RotateLastInputEvent
  (params (actor_rotation :type Rotator) (last_input_rot :type Rotator) (time :type Float%20%28single-precision%29))
  (bind _rotatelastinputtimeline (Variables|Default|GetRotateLastInputTimeline))
  ;[1 1 1] Rotation Interp to last input rotation with timeline
  (Audio|Components|Audio|Stop _rotatelastinputtimeline)
  (Components|Timeline|SetPlayRate _rotatelastinputtimeline time)
  (bind _새_트랙_0 (Timeline|RotateLastInputTimeline PlayFromStart)
    (:Update
      (Transformation|SetActorRotation (Math|Interpolation|Ease "ExpoOut" _새_트랙_0 actor_rotation last_input_rot true) true))))

(event Custom|SetStateMulticast
  (params (NewParam :type CharacterState%20Enum :default "NewEnumerator0"))
  ;[1 1 1] Character state change ( multicast )
  (캐릭터상태제어|SetState NewParam))

(event Custom|RagdollSetMult
  (bind _ragdollserverlocation (Variables|래그돌관련|GetRagdollServerLocation))
  ;[1 1 1] 래그돌 세팅 멀티캐스트
  (if (Ability|HasAuthority)
    (if (Pawn|IsPlayerControlled)
      (Variables|래그돌관련|SetPrevRagdollServerLocation _ragdollserverlocation :!label _label)
      (Variables|래그돌관련|SetLastRagdollServerLocation _ragdollserverlocation)
      (Variables|래그돌관련|Setreplication%20delay%20count 0.0)
      (Variables|래그돌관련|SetRagdollOnGround false)
      (Pawn|Components|CharacterMovement|SetMovementMode (Variables|Character|GetCharacterMovement) "MOVE_None" 0)
      (Collision|SetCollisionEnabled (Variables|Collision|GetCapsuleComponent) "QueryOnly")
      (Collision|SetCollisionEnabled (Variables|Character|GetMesh) "QueryAndPhysics")
      (Class|SkeletalMeshComponent|SetAllBodiesBelowSimulatePhysics (Variables|Character|GetMesh) (Variables|캐릭터상태관련|GetBoneName-Ragdoll) true true)
      (Variables|캐릭터상태관련|SetState "NewEnumerator4")
      (Class|AnimInstance|MontageStopGroupbyName (Variables|Default|GetMainAnimInstance) 0.0 "DefaultGroup")
      (else
        (Variables|캐릭터상태관련|SetState "NewEnumerator4")
        (Pawn|Components|CharacterMovement|SetMovementMode (Variables|Character|GetCharacterMovement) "MOVE_None" 0)
        (Class|AnimInstance|MontageStopGroupbyName (Variables|Default|GetMainAnimInstance) 0.0 "DefaultGroup")))
    (else
      (goto _label))))

(event Game|Damage|EventAnyDamage
  (params (Damage :type Float%20%28single-precision%29) (DamageType :type Damage%20Type%20Object%20Reference) (InstigatedBy :type Controller%20Object%20Reference) (DamageCauser :type Actor%20Object%20Reference))
  (Development|PrintString (Utilities|String|ToString(Float) Damage))
  (Audio|SpawnSoundatLocation "/Game/Blueprint/SQ_Hit.SQ_Hit" (Transformation|GetActorLocation) "0, 0, 0" 1.0 1.0 0.0 0 0)
  (Animation|PlayAnimMontage "/Game/Animation/Actions/Hit_F_Montage.Hit_F_Montage" 1.0 "None"))

(event Collision|EventHit
  (params (MyComp :type Primitive%20Component%20Object%20Reference) (Other :type Actor%20Object%20Reference) (OtherComp :type Primitive%20Component%20Object%20Reference) (bSelfMoved :type Boolean) (HitLocation :type Vector :default "0, 0, 0") (HitNormal :type Vector :default "0, 0, 0") (NormalImpulse :type Vector :default "0, 0, 0") (Hit :type Hit%20Result%20Structure%20%28by%20ref%29))
  ;[1 1 1] 액터 히트 이벤트
  (switch Utilities|FlowControl|Switch|SwitchonCharacterState (Variables|캐릭터상태관련|GetState)
    (:NewEnumerator2
      _)
    (:NewEnumerator4
      _))
  (if (not (Variables|래그돌관련|GetRagdollOnGround))
    (이펙트|DustEffect HitLocation)))

(event EventRotateActor
  (params (target_rotation :type Rotator :default "0, 0, 0") (time :type Float%20%28single-precision%29))
  (bind _rotatelastinputtimeline (Variables|Default|GetRotateLastInputTimeline))
  (bind _output_get (Variables|Default|Settmp_rotation (Transformation|GetActorRotation)))
  (Audio|Components|Audio|Stop _rotatelastinputtimeline)
  (Components|Timeline|SetPlayRate _rotatelastinputtimeline (/ 1.0 time))
  (bind _새_트랙_0 (Timeline|타임라인_0 PlayFromStart)
    (:Update
      (Transformation|SetActorRotation (Math|Interpolation|Ease "ExpoOut" _새_트랙_0 _output_get target_rotation true) true))))

(event EventSetDamageData
  (params (damage_data :type Damage%20Data%20Structure))
  (Variables|공격관련|Setdamage_data damage_data))

(event Custom|CtoS-TargetLocation
  (params (RagdollServerLocation :type Vector))
  ;[1 0.5156 0.5156] Client ragdoll Move to server's ragdoll location with interpolation and actor location & rotation adjust
  ;;[1 1 1] 서버 : 소유 클라이언트로 부터 위치를 전달받으면 변수를 업데이트해서 리플리케이트
  (bind _output_get (Variables|래그돌관련|SetRagdollServerLocation RagdollServerLocation))
  (래그돌시스템|StickontheGround _output_get))

(event Custom|SwitchState
  (bind _mesh (Variables|Character|GetMesh))
  ;[1 0.5156 0.5156] Client ragdoll Move to server's ragdoll location with interpolation and actor location & rotation adjust
  ;;[1 1 1] 래그돌의 위치를 옮길 수 있게 피직스 핸들로 엉덩이를 잡음
  (Utilities|FlowControl|DoOnce false) ; enters at Reset
)

(event EventTick
  (params (DeltaSeconds :type Float%20%28single-precision%29))
  (bind _mesh (Variables|Character|GetMesh))
  (Utilities|FlowControl|Sequence
    (:then_0
      ;[1 1 1] Set Pitch and Yaw
      (CallFunction|Look))
    (:then_1
      (switch Utilities|FlowControl|Switch|SwitchonCharacterState (Variables|캐릭터상태관련|GetState)
        (:NewEnumerator4
          ;[1 0.5156 0.5156] Client ragdoll Move to server's ragdoll location with interpolation and actor location & rotation adjust
          (Utilities|FlowControl|Sequence
            (:then_0
              ;;[1 1 1] 자동 위치 동기화 종료
              (Utilities|FlowControl|DoOnce false :!label _label
                (:Completed
                  (Class|Actor|SetReplicateMovement false))))
            (:then_1
              (Networking|SwitchHasAuthority
                (:Authority
                  ;[1 1 1] 리슨 서버일때 로직
                  (if (not (Networking|IsDedicatedServer))
                    (if (Pawn|IsLocallyControlled)
                      (bind _output_get (Variables|래그돌관련|SetRagdollServerLocation (Transformation|GetSocketLocation (Variables|Character|GetMesh) "pelvis")))
                      (래그돌시스템|StickontheGround _output_get)
                      (else
                        (Utilities|FlowControl|Sequence :!label _label_2
                          (:then_0
                            ;;[1 1 1] 서버위 위치가 갱신되었는지에 따라 보간 파라미터와 주기 조정
                            (if (Class|KismetMathLibrary|EqualExactlyVectorVector (Variables|래그돌관련|GetLastRagdollServerLocation) (Variables|래그돌관련|GetRagdollServerLocation))
                              (Variables|래그돌관련|Setreplication%20delay%20count (+ (Variables|래그돌관련|Getreplication%20delay%20count) DeltaSeconds))
                              (else
                                (Variables|래그돌관련|Setlast%20update%20delay (Variables|래그돌관련|Getreplication%20delay%20count))
                                (Variables|래그돌관련|Setreplication%20delay%20count DeltaSeconds)
                                (Variables|래그돌관련|SetPrevRagdollServerLocation (Variables|래그돌관련|GetLastRagdollServerLocation)))))
                          (:then_1
                            ;;[1 1 1] 래그돌의 위치를 옮길 수 있게 피직스 핸들로 엉덩이를 잡음
                            (Utilities|FlowControl|DoOnce false
                              (:Completed
                                (Class|PhysicsHandleComponent|GrabComponentatLocation (Variables|Default|GetPhysicsHandle) _mesh "pelvis" (Transformation|GetSocketLocation _mesh "pelvis")))))
                          (:then_2
                            ;;[1 1 1] 서버 위치로 피직스 핸들로 래그돌의 엉덩이를 잡아끌고 보간된 위치로 액터를 이동시킴
                            (Physics|Components|PhysicsHandle|SetTargetLocation (Variables|Default|GetPhysicsHandle) (Variables|래그돌관련|GetRagdollServerLocation))
                            (래그돌시스템|StickontheGround (Math|Interpolation|Ease "Linear" (Math|Float|Min(Float) (/ (Variables|래그돌관련|Getreplication%20delay%20count) (Variables|래그돌관련|Getlast%20update%20delay)) 1.0) (Variables|래그돌관련|GetPrevRagdollServerLocation) (Variables|래그돌관련|GetRagdollServerLocation)))
                            (Variables|래그돌관련|SetLastRagdollServerLocation (Variables|래그돌관련|GetRagdollServerLocation))))))))
                (:Remote
                  (if (Pawn|IsLocallyControlled)
                    ;;[1 1 1] 소유클라이언트 : 래그돌의 위치로 액터를 이동시키고 서버에서 위치를 리플리케이트 할 수 있도록 서버로 전달
                    (bind _output_get_2 (Variables|래그돌관련|SetRagdollServerLocation (Transformation|GetSocketLocation (Variables|Character|GetMesh) "pelvis")))
                    (래그돌시스템|StickontheGround _output_get_2)
                    (CallFunction|CtoS-TargetLocation _output_get_2)
                    (else
                      (goto _label_2))))))))
        (:NewEnumerator5
          (goto _label Reset))))))

(event EventBeginPlay
  (bind _mesh (Variables|Character|GetMesh))
  (bind _returnvalue (Components|SkeletalMesh|GetAnimInstance _mesh))
  (Utilities|FlowControl|Sequence
    (:then_0
      ;[1 1 1] 데디케이티드 서버와 소유 클라이언트는 핸들을 사용하지 않을 것이기 때문에 디스트로이
      (Networking|SwitchHasAuthority
        (:Authority
          (if (Networking|IsDedicatedServer)
            (Components|DestroyComponent (Variables|Default|GetPhysicsHandle) :!label _label)
            (else
              (if (Pawn|IsLocallyControlled) :!label _label_2
                (goto _label)))))
        (:Remote
          (goto _label_2))))
    (:then_1
      ;[1 1 1] Set main anim instance
      (if (Utilities|IsValid _returnvalue)
        (Variables|Default|SetMainAnimInstance _returnvalue)))))

(event EventLook
  (Variables|바라보기관련|Setlook_pitch (Math|Float|ClampAngle (.Pitch (Math|Rotator|BreakRotator (Math|Interpolation|RInterpTo (Math|Rotator|MakeRotator 0.0 (Variables|바라보기관련|Getlook_pitch) (Variables|바라보기관련|Getlook_yaw)) (Math|Rotator|Delta(Rotator) (Variables|Default|GetR_look_rotation) (Transformation|GetActorRotation)) (Utilities|Time|GetWorldDeltaSeconds) 15.0))) -9e+01 9e+01))
  (Variables|바라보기관련|Setlook_yaw (Math|Float|ClampAngle (.Yaw (Math|Rotator|BreakRotator (Math|Interpolation|RInterpTo (Math|Rotator|MakeRotator 0.0 (Variables|바라보기관련|Getlook_pitch) (Variables|바라보기관련|Getlook_yaw)) (Math|Rotator|Delta(Rotator) (Variables|Default|GetR_look_rotation) (Transformation|GetActorRotation)) (Utilities|Time|GetWorldDeltaSeconds) 15.0))) -9e+01 9e+01)))

(fn ConstructionScript
  ;[1 1 1] Foot IK setup
  (Variables|Default|SetIKTraceDistance (* (.Z (Math|Vector|BreakVector (.Scale (Math|Transform|BreakTransform (Transformation|GetActorTransform))))) (Variables|/Script/Engine.CapsuleComponent|GetCapsuleHalfHeight (Variables|Collision|GetCapsuleComponent)))))

(fn GetonSprint
  (return (Variables|캐릭터상태관련|GetOnSprint self)))

(fn DodgeStart
  (bind _charactermovement (Variables|Character|GetCharacterMovement))
  (Variables|/Script/Engine.CharacterMovementComponent|SetMaxWalkSpeed _charactermovement 1.4e+03)
  (Variables|/Script/Engine.CharacterMovementComponent|SetMaxAcceleration _charactermovement 1e+04))

(fn DodgeEnd
  (bind _charactermovement (Variables|Character|GetCharacterMovement))
  (Variables|캐릭터상태관련|SetDodgeChk false)
  (Variables|/Script/Engine.CharacterMovementComponent|SetMaxAcceleration _charactermovement 2048.0)
  (if (Variables|캐릭터상태관련|GetOnSprint)
    (Variables|/Script/Engine.CharacterMovementComponent|SetMaxWalkSpeed _charactermovement (Variables|캐릭터속도관련|GetSprintSpeed))
    (else
      (Variables|/Script/Engine.CharacterMovementComponent|SetMaxWalkSpeed _charactermovement (Variables|캐릭터속도관련|GetWalkSpeed)))))

(fn SetAdditionalSpeedRate
  (params (Rate :type Float%20%28single-precision%29))
  (bind _charactermovement (Variables|Character|GetCharacterMovement))
  (bind _walkspeed (Variables|캐릭터속도관련|GetWalkSpeed))
  (Networking|SwitchHasAuthority
    (:Authority
      (Variables|캐릭터속도관련|SetAdditionalSpeedRate Rate)
      (Variables|/Script/Engine.CharacterMovementComponent|SetMaxWalkSpeed _charactermovement (+ (* Rate 2e+03) _walkspeed)))
    (:Remote
      (Variables|/Script/Engine.CharacterMovementComponent|SetMaxWalkSpeed _charactermovement (+ (* (Variables|캐릭터속도관련|GetAdditionalSpeedRate) 8e+02) _walkspeed)))))

(fn AttackEnd
  (Variables|캐릭터상태관련|SetAttackNum 0)
  (Variables|캐릭터상태관련|SetState "NewEnumerator0")
  (Pawn|Components|CharacterMovement|SetMovementMode (Variables|Character|GetCharacterMovement) "MOVE_Walking" 0))

(fn StateChk
  (params (State :type CharacterState%20Enum :default "NewEnumerator0"))
  (return (Utilities|Enum|Equal(Enum) (Variables|캐릭터상태관련|GetState) State)))

(fn ChracterMovementModeChange
  (params (TargetMode :type EMovementMode%20Enum :default "MOVE_None"))
  (Pawn|Components|CharacterMovement|SetMovementMode (Variables|Character|GetCharacterMovement) TargetMode 0))

(fn GetState
  (return (Variables|캐릭터상태관련|GetState)))

(fn SetState
  (params (TargetState :type CharacterState%20Enum :default "NewEnumerator0"))
  (if (Utilities|Enum|NotEqual(Enum) TargetState (Variables|캐릭터상태관련|GetState))
    (CallFunction|SwitchState)
    (Utilities|FlowControl|Sequence
      (:then_0
        (switch Utilities|FlowControl|Switch|SwitchonCharacterState TargetState
          (:NewEnumerator0
            ;[1 1 1] State -> Walk_Run_Jump
            (Pawn|Components|CharacterMovement|SetMovementMode (Variables|Character|GetCharacterMovement) "MOVE_Walking" 0)
            (Collision|SetCollisionEnabled (Variables|Collision|GetCapsuleComponent) "QueryAndPhysics")
            (Collision|SetCollisionEnabled (Variables|Character|GetMesh) "QueryOnly")
            (Variables|캐릭터상태관련|SetState "NewEnumerator0"))
          (:NewEnumerator1
            ;[1 1 1] State -> Attack
            (Class|Pawn|ConsumeMovementInputVector)
            (Pawn|Components|CharacterMovement|DisableMovement (Variables|Character|GetCharacterMovement))
            (Variables|캐릭터상태관련|SetState "NewEnumerator1"))
          (:NewEnumerator2
            ;[1 1 1] State -> Airbone
            (bind _chk (CallFunction|StateChk "NewEnumerator4"))
            (if _chk
              (return)
              (else
                (Variables|캐릭터상태관련|SetDodgeChk false)
                (Variables|캐릭터상태관련|SetOnSprint false)
                (Variables|공격관련|SetOnAction false)
                (래그돌시스템|AriboneStart)
                (Variables|캐릭터상태관련|SetState "NewEnumerator2"))))
          (:NewEnumerator4
            ;[1 1 1] State -> Ragdoll
            (Utilities|FlowControl|Sequence
              (:then_0
                (Variables|캐릭터상태관련|SetDodgeChk false)
                (Variables|캐릭터상태관련|SetOnSprint false)
                (Variables|공격관련|SetOnAction false)
                (CallFunction|RagdollSetonServer))))
          (:NewEnumerator5
            ;[1 1 1] 일어서기
            (래그돌시스템|RagdollGetupInit)
            (Variables|캐릭터상태관련|SetState "NewEnumerator5")))))))

(fn AriboneStart
  (bind _returnvalue (Transformation|GetVelocity))
  (bind _mainaniminstance (Variables|Default|GetMainAnimInstance))
  (bind _mesh (Variables|Character|GetMesh))
  (bind _returnvalue_2 (Math|Vector|VectorLength _returnvalue))
  (bind _returnvalue_3 (/ _returnvalue_2 2e+03))
  (Collision|SetCollisionEnabled (Variables|Collision|GetCapsuleComponent) "QueryAndPhysics")
  (Collision|SetCollisionObjectType _mesh "ECC_PhysicsBody")
  (Collision|SetCollisionEnabled _mesh "QueryAndPhysics")
  (Class|SkeletalMeshComponent|SetAllBodiesBelowSimulatePhysics _mesh (Variables|캐릭터상태관련|GetBoneName-Ragdoll) true false)
  (if (> (* (.X (Math|Vector|BreakVector _returnvalue)) (.X (Math|Vector|BreakVector (Transformation|GetActorForwardVector)))) 0.0)
    (Animation|Montage|MontagePlay _mainaniminstance "/Game/Animation/Airbone_b_Montage.Airbone_b_Montage" (* _returnvalue_3 -1.0) "MontageLength" 0.0 true)
    (else
      (Animation|Montage|MontagePlay _mainaniminstance "/Game/Animation/Airbone_b_Montage.Airbone_b_Montage" _returnvalue_3 "MontageLength" 0.0 true))))

(fn RagdollEnd
  (params (InterpolationRate :type Float%20%28single-precision%29))
  (bind _mesh (Variables|Character|GetMesh))
  (Collision|SetCollisionEnabled (Variables|Collision|GetCapsuleComponent) "QueryAndPhysics")
  (Collision|SetCollisionEnabled _mesh "NoCollision")
  (Physics|SetSimulatePhysics _mesh false))

(fn RagdollGetup
  (params (InterpolationRate :type Float%20%28single-precision%29))
  ;[1 1 1] 일어서는 애니메이션과 피직스를 블렌딩
  (Class|SkeletalMeshComponent|SetAllBodiesPhysicsBlendWeight (Variables|Character|GetMesh) (- 1.0 InterpolationRate) true)
  (Transformation|SetActorRotation (Math|Rotator|Lerp(Rotator) (Transformation|GetActorRotation) (Variables|래그돌관련|GetTargetRagdollRotation) InterpolationRate true)))

(fn RagdollGetupInit
  (bind _mesh (Variables|Character|GetMesh))
  (bind _returnvalue (Transformation|GetSocketRotation _mesh "pelvis"))
  (Utilities|FlowControl|Sequence
    (:then_0
      ;[1 1 1] 리플리케이션 다시 킴
      (Class|Actor|SetReplicateMovement true)
      (bind _mainaniminstance (Variables|Default|GetMainAnimInstance)
        (:then
          (Class|AnimInstance|SavePoseSnapshot _mainaniminstance "RagdollPose"))
        (:else)))
    (:then_1
      ;[1 1 1] 래그돌이 일어날 방향을 결정
      (bind _output_get (Variables|래그돌관련|SetRagdollFaceUp (< (.roll _returnvalue) 0.0)))
      (bind _output_get_2 (Variables|래그돌관련|SetTargetRagdollRotation (Math|Rotator|MakeRotator 0.0 0.0 (select _output_get (- (.yaw _returnvalue) 1.8e+02) (.yaw _returnvalue)))))
      (Transformation|SetActorRotation _output_get_2 true))
    (:then_2
      ;[1 1 1] 누워있는 방향에 맞게 일어서는 애니메이션 몽타주 플레이
      (Pawn|Components|CharacterMovement|SetMovementMode (Variables|Character|GetCharacterMovement) "MOVE_Walking" 0)
      (if (Variables|래그돌관련|GetRagdollFaceUp)
        (bind _mainaniminstance_2 (Variables|Default|GetMainAnimInstance)
          (:then
            (Animation|Montage|MontagePlay _mainaniminstance_2 "/Game/Animation/Actions/ALS_CLF_GetUp_Back_Montage_Default.ALS_CLF_GetUp_Back_Montage_Default" 1.0 "MontageLength" 0.0 true))
          (:else))
        (else
          (bind _mainaniminstance_3 (Variables|Default|GetMainAnimInstance)
            (:then
              (Animation|Montage|MontagePlay _mainaniminstance_3 "/Game/Animation/Actions/ALS_CLF_GetUp_Front_Montage_Default.ALS_CLF_GetUp_Front_Montage_Default" 1.0 "MontageLength" 0.0 true))
            (:else)))))
    (:then_3
      ;[1 1 1] 메쉬와 액터의 콜리전,피직스 설정 변환
      (Collision|SetCollisionEnabled (Variables|Collision|GetCapsuleComponent) "QueryAndPhysics")
      (Collision|SetCollisionEnabled (Variables|Character|GetMesh) "QueryOnly")
      (Physics|SetSimulatePhysics (Variables|Character|GetMesh) false))))

(fn RagdollUpdate
  (Utilities|FlowControl|Sequence
    (:then_0
      ;[1 1 1] Set the Last Ragdoll Velocity.
      (bind _returnvalue (Physics|GetPhysicsLinearVelocity (Variables|Character|GetMesh) "root"))
      (Variables|래그돌관련|SetLastRagdollVelocity _returnvalue))
    (:then_1
      ;[1 1 1] Use the Ragdoll Velocity to scale the ragdoll's joint strength for physical animation.
      (Class|SkeletalMeshComponent|SetAllMotorsAngularDriveParams (Variables|Character|GetMesh) (Math|Float|MapRangeClamped (Math|Vector|VectorLength (Variables|래그돌관련|GetLastRagdollVelocity)) 0.0 1e+03 0.0 2.5e+04) 0.0 0.0 false))))

(fn StickontheGround
  (params (Location :type Vector))
  (bind _mesh (Variables|Character|GetMesh))
  (bind _returnvalue (Transformation|GetSocketRotation _mesh "pelvis"))
  ;[1 1 1] 액터가 땅 속으로 안 박히게 라인 트레이스로 충돌 감지
  (bind _output_get (LocalVariables|Setsrc%20location Location))
  (bind _outhit (Collision|LineTraceByChannel _output_get (Math|Vector|MakeVector (.X (Math|Vector|BreakVector _output_get)) (.Y (Math|Vector|BreakVector _output_get)) (- (.Z (Math|Vector|BreakVector _output_get)) (Components|Capsule|GetScaledCapsuleHalfHeight (Variables|Collision|GetCapsuleComponent)))) "TraceTypeQuery1" false 0 "None"))
  (Utilities|FlowControl|Sequence
    (:then_0
      (if (and (not (Variables|래그돌관련|GetRagdollOnGround)) (.bblockinghit _outhit))
        (이펙트|DustEffect (.location _outhit))))
    (:then_1
      (bind _output_get_2 (Variables|래그돌관련|SetRagdollOnGround (.bblockinghit _outhit)))
      (if _output_get_2
        (bind _output_get_3 (Variables|래그돌관련|SetRagdollFaceUp (< (.roll _returnvalue) 0.0)))
        (Transformation|SetActorRotation (Math|Rotator|MakeRotator 0.0 0.0 (select _output_get_3 (- (.yaw _returnvalue) 1.8e+02) (.yaw _returnvalue))))
        (Transformation|SetActorLocation (Math|Vector|MakeVector (.X (Math|Vector|BreakVector (LocalVariables|Getsrc%20location))) (.Y (Math|Vector|BreakVector (LocalVariables|Getsrc%20location))) (+ (.Z (Math|Vector|BreakVector (LocalVariables|Getsrc%20location))) (- (Components|Capsule|GetScaledCapsuleHalfHeight (Variables|Collision|GetCapsuleComponent)) (Math|Float|Absolute(Float) (- (.z (.impactpoint _outhit)) (.z (.tracestart _outhit))))) 2.0)) false false)
        (else
          (Transformation|SetActorLocation (LocalVariables|Getsrc%20location) false false))))))

(fn GetCameraBoom
  (return (Transformation|GetActorLocation)))

(fn RotateLastInput
  (params (time :type Float%20%28single-precision%29) (last_movement_input :type Vector))
  (if (> (Math|Vector|VectorLength last_movement_input) 0.0)
    (CallFunction|RotateLastInputEvent (Transformation|GetActorRotation) (Math|Rotator|MakeRotfromX last_movement_input) (/ 1.0 time))))

(fn DustEffect
  (params (target_location :type Vector))
  (Audio|PlaySoundatLocation "/Game/SFX/THUD_Medium_01_mono.THUD_Medium_01_mono" target_location "0, 0, 0" 1.0 1.0 0.0 0 0 0)
  (AddComponent|AddNiagaraComponent false (Math|Transform|MakeTransform (- target_location (Transformation|GetActorLocation)))))

(fn GetWeapon)