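; Enemy AI controller that runs the BT_Enemy behavior tree on BeginPlay and manages the target it acts on.
; AI Perception updates write the perceived actor to the target_actor blackboard key only when no valid target is stored, without checking whether it was sensed or lost.
; A target_change event overwrites that key with a supplied target unconditionally.
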(event OnTargetPerceptionUpdated(AIPerception)
  (params (Actor :type Actor%20Object%20Reference) (Stimulus :type AI%20Stimulus%20Structure))
  (bind _returnvalue (Utilities|Name|MakeLiteralName "target_actor"))
  (bind _blackboard (Variables|Default|GetBlackboard))
  (Utilities|IsValid (AI|Components|Blackboard|GetValueasObject _blackboard _returnvalue)
    (:Is%20Not%20Valid
      (AI|Components|Blackboard|SetValueasObject _blackboard _returnvalue Actor))))

(event Custom|target_change
  (params (new_target :type Actor%20Object%20Reference))
  (AI|Components|Blackboard|SetValueasObject (Variables|Default|GetBlackboard) (Utilities|Name|MakeLiteralName "target_actor") new_target))

(event EventBeginPlay
  (AI|RunBehaviorTree "/Game/Blueprint/AI/BT_Enemy.BT_Enemy"))

(fn ConstructionScript)