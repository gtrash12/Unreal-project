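; Player controller that creates the local HUD and routes player input for quick slots, interaction and the inventory screen.
; Quick-slot presses look up the slotted item in game instance data and fire each effect through its class default object.
; Interaction requests go through a server event to the player character, while HUD events show or hide the prompt text.
; An item-use multicast plays a drink montage; older potion-use logic is left disconnected.
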(event Custom|Server_ItemUse
  (params (item_id :type Name) (actor :type Actor%20Object%20Reference))
  (CallFunction|MulticastItemUse actor))

(event Custom|Multicast_ItemUse
  (params (actor :type Actor%20Object%20Reference))
  (bind _asbase_character (Utilities|Casting|CastToBaseCharacter actor))
  (Class|InterfaceBaseCharacter|SetIsonAction(Message) actor true)
  (Animation|PlayAnimMontage _asbase_character "/Game/Animation/Combat/drink_Montage.drink_Montage" 1.0 "None"))

(event EventBeginPlay
  ;[1 1 1] widget setting
  (if (Pawn|IsLocalPlayerController)
    (Utilities|FlowControl|Sequence
      (:then_0
        (if (and (not (Networking|IsDedicatedServer)) (Pawn|IsLocalPlayerController))
          (bind _returnvalue (UserInterface|CreateWidget "/Game/Blueprint/Widget/Widget_UI.Widget_UI_C"))
          (bind _output_get (Variables|Default|SetHUD_reference _returnvalue))
          (UserInterface|Viewport|AddtoViewport _output_get 0))))))

(event EventShowInteractionText
  (params (__text :type Text%20%28by%20ref%29))
  (bind _hud_reference (Variables|Default|GetHUD_reference))
  ;[1 1 1] 인터랙션 오브젝트 텍스트 인터페이스
  (Utilities|IsValid _hud_reference
    (:Is%20Valid
      (Rendering|Components|TextRender|SetText (Variables|/Game/Blueprint/Widget/Widget_UI.Widget_UI_C|Gettext_left _hud_reference) __text)
      (Widget|SetVisibility (Variables|/Game/Blueprint/Widget/Widget_UI.Widget_UI_C|GetInteractBox _hud_reference) "Visible"))))

(event EventRemoveInteractionText
  (bind _hud_reference (Variables|Default|GetHUD_reference))
  ;[1 1 1] 인터랙션 오브젝트 텍스트 인터페이스
  (Utilities|IsValid _hud_reference
    (:Is%20Valid
      (Widget|SetVisibility (Variables|/Game/Blueprint/Widget/Widget_UI.Widget_UI_C|GetInteractBox _hud_reference) "Collapsed"))))

(event Input|ActionEvents|InputActionUseQuickSlot
  (params (Key :type Key%20Structure :default "None"))
  (:Pressed
    (bind _returnvalue (Class|ControllerPlayer|GetRegisteredQuickSlotInvenIndex Key))
    (if (>= _returnvalue 0)
      (bind _returnvalue_2 (Class|ControllerPlayer|GetInventoryData _returnvalue))
      (bind _aspwogame_instance (Utilities|Casting|CastToPWOGameInstance (Game|GetGameInstance)))
      (bind _returnvalue_3 (Class|PWOGameInstance|FindItemData _aspwogame_instance (.item_id (Utilities|Struct|BreakInventoryData _returnvalue_2))))
      (for _array_element (.item_effect_list (Utilities|Struct|BreakItemData _returnvalue_3))
        (bind _returnvalue_4 (Class|CustomBPFunctionLibrary|GetClassDefaultObject (.item_effect (Utilities|Struct|BreakItemEffect _array_element))))
        (Variables|/Script/CyperArena.BaseItemEffect|Setvalue _returnvalue_4 (.value (Utilities|Struct|BreakItemEffect _array_element)))
        (bind _ascharacter (Utilities|Casting|CastToCharacter (Game|Player|GetPlayerPawn 0)))
        (Class|InterfaceItemEffect|OnActivate(Message) _returnvalue_4 _ascharacter _returnvalue)))))

(event Custom|Server-interaction
  (params (target :type Actor%20Object%20Reference) (causor :type Actor%20Object%20Reference))
  (bind _asbp_player_character_cpp (Utilities|Casting|CastToBP_PlayerCharacter_cpp causor))
  (Default|Interact _asbp_player_character_cpp target causor))

(event Input|ActionEvents|InputActionInteraction
  (params (Key :type Key%20Structure))
  (bind _interaction_target (Variables|Default|Getinteraction_target))
  (:Pressed
    (Utilities|IsValid _interaction_target
      (:Is%20Valid
        (CallFunction|Server-interaction _interaction_target (Game|Player|GetPlayerPawn 0))))))

(event Input|ActionEvents|InputActionToggleInventory
  (params (Key :type Key%20Structure))
  (:Pressed
    (bind _returnvalue (UserInterface|CreateWidget "/Game/Blueprint/Widget/Widget_Inventory.Widget_Inventory_C" self))
    (UserInterface|Viewport|AddtoViewport _returnvalue 0)
    (Variables|Default|SetbShowMouseCursor true)
    (Input|SetInputModeUIOnly self _returnvalue "DoNotLock")))

(fn ConstructionScript)