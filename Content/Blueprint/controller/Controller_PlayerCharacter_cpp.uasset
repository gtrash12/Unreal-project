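; Player controller that spawns a smoothed follow camera and local HUD and handles lock-on, interaction, potion quick slot and inventory input.
; Lock-on picks visible enemies nearest the camera's aim by dot product, switching sideways on axis input with a cooldown.
; Tick traces ahead for "interactable" actors to show prompts.
; Interactions and potion use go through server-then-multicast events; damage is relayed via the server.
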(event Custom|Server_ItemUse
  (params (item_id :type Name) (actor :type Actor%20Object%20Reference))
  (CallFunction|MulticastItemUse actor))

(event Custom|Multicast_ItemUse
  (params (actor :type Actor%20Object%20Reference))
  (bind _asbase_character (Utilities|Casting|CastToBaseCharacter actor))
  (Class|InterfaceBaseCharacter|SetIsonAction(Message) actor true)
  (Animation|PlayAnimMontage _asbase_character "/Game/Animation/Combat/drink_Montage.drink_Montage" 1.0 "None"))

(event Custom|Server_ApplyDamage
  (params (damaged_actor :type Actor%20Object%20Reference) (damage_id :type Name) (damage_causer :type Actor%20Object%20Reference) (hit_bone_name :type Name))
  (Class|InterfaceBaseCharacter|ApplyDamage(Message) damaged_actor damage_id damage_causer hit_bone_name))

(event EventBeginPlay
  (bind _returnvalue (Game|Player|GetPlayerPawn 0))
  (bind _returnvalue_2 (Game|GetPlayerCameraManager 0))
  (Utilities|FlowControl|Sequence
    (:then_0
      ;[1 1 1] widget setting
      (if (and (not (Networking|IsDedicatedServer)) (Pawn|IsLocalPlayerController))
        (bind _returnvalue_3 (UserInterface|CreateWidget "/Game/Blueprint/Widget/Widget_UI.Widget_UI_C"))
        (bind _output_get (Variables|Default|SetHUD_reference _returnvalue_3))
        (UserInterface|Viewport|AddtoViewport _output_get 0)))
    (:then_1
      ;[1 1 1] Spawn and set Smooth Camera
      (Class|PlayerCameraManager|SetManualCameraFade :self _returnvalue_2 :InFadeAmount 1.0 :bInFadeAudio true)
      (Utilities|FlowControl|Delay 2.0)
      (CameraFades|StartCameraFade :self _returnvalue_2 :FromAlpha 1.0 :Duration 2.0 :bShouldFadeAudio true)
      (bind _returnvalue_4 (Game|SpawnActorfromClass "/Game/Blueprint/Camera_BP.Camera_BP_C" (Transformation|GetActorTransform _returnvalue) "Undefined" 0 0))
      (Variables|/Game/Blueprint/Camera_BP.Camera_BP_C|SetTarget _returnvalue_4 _returnvalue)
      (Game|Player|SetViewTargetwithBlend (Game|GetPlayerController 0) _returnvalue_4 0.0 "VTBlend_Linear" 0.0 false)
      (Variables|Default|Setfollow_cam _returnvalue_4))))

(event EventCtoSApplyDamage
  (params (damaged_actor :type Actor%20Object%20Reference) (__damage_id :type Name :default "None") (damage_causer :type Actor%20Object%20Reference) (__hit_bone_name :type Name :default "None"))
  (CallFunction|ServerApplyDamage damaged_actor __damage_id damage_causer __hit_bone_name))

(event Input|ActionEvents|InputActionQuickSlot1
  (params (Key :type Key%20Structure :default "None"))
  (bind _returnvalue (Game|Player|GetPlayerPawn 0))
  (:Pressed
    (bind _asbase_character (Utilities|Casting|CastToBaseCharacter _returnvalue))
    (if (and (not (Variables|/Script/CyperArena.BaseCharacter|Getis_on_action _asbase_character)) (> (Variables|Default|Getpotion_count) 0))
      (CallFunction|ServerItemUse "hp_portion1" _returnvalue))))

(event Custom|Server-interaction
  (params (target :type Actor%20Object%20Reference) (causor :type Actor%20Object%20Reference))
  (CallFunction|Multicast-interaction target causor))

(event Custom|Multicast-interaction
  (params (target :type Actor%20Object%20Reference) (causor :type Actor%20Object%20Reference))
  (Utilities|Casting|CastToBP_PlayerCharacter_cpp (Game|Player|GetPlayerPawn 0))
  (bind _aspwogame_instance (Utilities|Casting|CastToPWOGameInstance (Game|GetGameInstance)))
  (Class|PWOGameInstance|Interact _aspwogame_instance target causor))

(event EventTick
  (params (DeltaSeconds :type Float%20%28single-precision%29))
  (bind _returnvalue (Game|Player|GetPlayerPawn 0))
  (bind _returnvalue_2 (Game|Player|GetPlayerPawn 0))
  (bind _follow_cam (Variables|Default|Getfollow_cam))
  (bind _returnvalue_3 (Transformation|GetActorLocation _returnvalue_2))
  (|CallParentFunction DeltaSeconds)
  (Variables|Default|Setlock_on_cooltime (- (Variables|Default|Getlock_on_cooltime) DeltaSeconds))
  (if (and (Pawn|IsLocalPlayerController) (Utilities|IsValid _follow_cam))
    (bind (_outhit _returnvalue_4) (Collision|LineTraceByChannel _returnvalue_3 (+ _returnvalue_3 (* (Transformation|GetActorForwardVector _follow_cam) 7e+01)) "TraceTypeQuery6" false 0 "None"))
    (if _returnvalue_4
      (if (Actor|ActorHasTag (.HitActor (Collision|BreakHitResult _outhit)) "interactable")
        (if (!= (.HitActor (Collision|BreakHitResult _outhit)) (Variables|Default|Getinteraction_target))
          (Utilities|IsValid (Variables|Default|Getinteraction_target)
            (:Is%20Valid
              (Class|InterfaceGeneral|RemoveInteractionInfo(Message) (Variables|Default|Getinteraction_target) _returnvalue))
            (:Is%20Not%20Valid
              _))
          (bind _output_get (Variables|Default|Setinteraction_target (.HitActor (Collision|BreakHitResult _outhit))))
          (Class|InterfaceGeneral|PopInteractionInfo(Message) _output_get _returnvalue))
        (else
          (Utilities|IsValid (Variables|Default|Getinteraction_target) :!label _label
            (:Is%20Valid
              (Class|InterfaceGeneral|RemoveInteractionInfo(Message) _output_get _returnvalue)
              (Variables|Default|Setinteraction_target 0)))))
      (else
        (goto _label)))))

(event EventReleaseLockON
  (bind _follow_cam (Variables|Default|Getfollow_cam))
  (bind _follow_cam_2 (Variables|Default|Getfollow_cam))
  (bind _follow_cam_3 (Variables|Default|Getfollow_cam))
  (Utilities|IsValid _follow_cam_2
    (:Is%20Valid
      (Variables|/Game/Blueprint/Camera_BP.Camera_BP_C|Setlock_on _follow_cam_2 true)
      (Variables|Default|Setlock_on true)
      (if (Variables|/Game/Blueprint/Camera_BP.Camera_BP_C|Getlock_on _follow_cam)
        (Variables|/Game/Blueprint/Camera_BP.Camera_BP_C|Setlock_on _follow_cam false)
        (Variables|Default|Setlock_on false)
        (Utilities|IsValid (Variables|/Game/Blueprint/Camera_BP.Camera_BP_C|Getlock_on_target (Variables|Default|Getfollow_cam))
          (:Is%20Valid
            (Class|BPIAI|SetLockonMarker(Message) (Variables|/Game/Blueprint/Camera_BP.Camera_BP_C|Getlock_on_target (Variables|Default|Getfollow_cam)) false))
          (:Is%20Not%20Valid
            _))
        (Pawn|SetControlRotation (Transformation|GetSocketRotation (Variables|/Game/Blueprint/Camera_BP.Camera_BP_C|GetCamera (Variables|Default|Getfollow_cam)) "None"))
        (else
          (bind _target (CallFunction|FindLockonTarget))
          (Utilities|IsValid _target
            (:Is%20Valid
              (Class|BPIAI|SetStateBarVisibility(Message) _target true)
              (Class|BPIAI|SetLockonMarker(Message) _target true)
              (Variables|/Game/Blueprint/Camera_BP.Camera_BP_C|Setlock_on _follow_cam_3 true)
              (Variables|Default|Setlock_on true)
              (Variables|/Game/Blueprint/Camera_BP.Camera_BP_C|Setlock_on_target _follow_cam_3 _target))))))))

(event Input|ActionEvents|InputActionLockOn
  (params (Key :type Key%20Structure :default "None"))
  (bind _follow_cam (Variables|Default|Getfollow_cam))
  (bind _follow_cam_2 (Variables|Default|Getfollow_cam))
  (:Pressed
    (Utilities|IsValid _follow_cam
      (:Is%20Valid
        (if (Variables|/Game/Blueprint/Camera_BP.Camera_BP_C|Getlock_on _follow_cam)
          (Variables|/Game/Blueprint/Camera_BP.Camera_BP_C|Setlock_on _follow_cam false)
          (Variables|Default|Setlock_on false)
          (Utilities|IsValid (Variables|/Game/Blueprint/Camera_BP.Camera_BP_C|Getlock_on_target (Variables|Default|Getfollow_cam))
            (:Is%20Valid
              (Class|BPIAI|SetLockonMarker(Message) (Variables|/Game/Blueprint/Camera_BP.Camera_BP_C|Getlock_on_target (Variables|Default|Getfollow_cam)) false))
            (:Is%20Not%20Valid
              _))
          (Pawn|SetControlRotation (Transformation|GetSocketRotation (Variables|/Game/Blueprint/Camera_BP.Camera_BP_C|GetCamera (Variables|Default|Getfollow_cam)) "None"))
          (else
            (bind _target (CallFunction|FindLockonTarget))
            (Utilities|IsValid _target
              (:Is%20Valid
                (Class|BPIAI|SetStateBarVisibility(Message) _target true)
                (Class|BPIAI|SetLockonMarker(Message) _target true)
                (Variables|/Game/Blueprint/Camera_BP.Camera_BP_C|Setlock_on _follow_cam_2 true)
                (Variables|Default|Setlock_on true)
                (Variables|/Game/Blueprint/Camera_BP.Camera_BP_C|Setlock_on_target _follow_cam_2 _target)))))))))

(event Input|ActionEvents|InputActionInteraction
  (params (Key :type Key%20Structure :default "None"))
  (bind _interaction_target (Variables|Default|Getinteraction_target))
  (:Pressed
    (Utilities|IsValid _interaction_target
      (:Is%20Valid
        (CallFunction|Server-interaction _interaction_target (Game|Player|GetPlayerPawn 0))))))

(event Input|ActionEvents|InputActionToggleInventory
  (params (Key :type Key%20Structure :default "None"))
  (:Pressed
    (bind _returnvalue (UserInterface|CreateWidget "/Game/Blueprint/Widget/Widget_Inventory.Widget_Inventory_C" self))
    (UserInterface|Viewport|AddtoViewport _returnvalue 0)
    (Variables|Default|SetbShowMouseCursor true)
    (Input|SetInputModeUIOnly self _returnvalue "DoNotLock")))

(event Input|AxisEvents|InputAxisChangeLockOn
  (params (AxisValue :type Float%20%28single-precision%29))
  (bind _follow_cam (Variables|Default|Getfollow_cam))
  (if (< (Variables|Default|Getlock_on_cooltime) 0.0)
    (Utilities|IsValid _follow_cam
      (:Is%20Valid
        (if (Variables|/Game/Blueprint/Camera_BP.Camera_BP_C|Getlock_on _follow_cam)
          (bind _target (CallFunction|ChangeLockonTarget AxisValue))
          (Utilities|IsValid _target
            (:Is%20Valid
              (Class|BPIAI|SetLockonMarker(Message) (Variables|/Game/Blueprint/Camera_BP.Camera_BP_C|Getlock_on_target (Variables|Default|Getfollow_cam)) false)
              (Class|BPIAI|SetStateBarVisibility(Message) _target true)
              (Class|BPIAI|SetLockonMarker(Message) _target true)
              (Variables|/Game/Blueprint/Camera_BP.Camera_BP_C|Setlock_on_target (Variables|Default|Getfollow_cam) _target)
              (Variables|Default|Setlock_on_cooltime 0.2))))))))

(fn ConstructionScript)

(fn FindLockonTarget
  (bind _follow_cam (Variables|Default|Getfollow_cam))
  (bind _camera (Variables|/Game/Blueprint/Camera_BP.Camera_BP_C|GetCamera _follow_cam))
  (bind _returnvalue (Transformation|GetSocketLocation _camera "None"))
  (bind _outactors (Actor|GetAllActorsOfClass "/Game/Blueprint/Character/BP_BaseEnemy.BP_BaseEnemy_C"))
  (for _array_element _outactors
    (bind _returnvalue_2 (Collision|LineTraceByChannel _returnvalue (Transformation|GetActorLocation _array_element) "TraceTypeQuery1" false _outactors "None"))
    (if (not _returnvalue_2)
      (Utilities|IsValid (Variables|/Game/Blueprint/Character/BP_BaseEnemy.BP_BaseEnemy_C|GetLockOnMarker _array_element)
        (:Is%20Valid
          (if (> (Math|Vector|DotProduct (Math|Vector|Normalize (Math|Vector|GetForwardVector (Math|Rotator|FindLookatRotation _returnvalue (Transformation|GetActorLocation _array_element)))) (Math|Vector|Normalize (Math|Vector|GetForwardVector (Transformation|GetSocketRotation _camera "None")))) (LocalVariables|Getmin_angle))
            (LocalVariables|Setmin_angle (Math|Vector|DotProduct (Math|Vector|Normalize (Math|Vector|GetForwardVector (Math|Rotator|FindLookatRotation _returnvalue (Transformation|GetActorLocation _array_element)))) (Math|Vector|Normalize (Math|Vector|GetForwardVector (Transformation|GetSocketRotation _camera "None")))))
            (LocalVariables|Setlock_on_target _array_element)
            (LocalVariables|Setmin_distance (Math|Vector|Distance(Vector) _returnvalue (Transformation|GetActorLocation _array_element))))))))
  (return (LocalVariables|Getlock_on_target)))

(fn ChangeLockonTarget
  (params (direction :type Float%20%28single-precision%29))
  (bind _follow_cam (Variables|Default|Getfollow_cam))
  (bind _camera (Variables|/Game/Blueprint/Camera_BP.Camera_BP_C|GetCamera _follow_cam))
  (LocalVariables|Setsocket_location (Transformation|GetSocketLocation _camera "None"))
  (LocalVariables|Setsocket_rotation (Transformation|GetSocketRotation _camera "None"))
  (LocalVariables|Settarget_foward_vector (Math|Vector|GetForwardVector (Math|Rotator|FindLookatRotation (LocalVariables|Getsocket_location) (Transformation|GetActorLocation (Variables|/Game/Blueprint/Camera_BP.Camera_BP_C|Getlock_on_target (Variables|Default|Getfollow_cam))))))
  (bind _outactors (Actor|GetAllActorsOfClass "/Game/Blueprint/Character/BP_BaseEnemy.BP_BaseEnemy_C"))
  (for _array_element _outactors
    (if (!= (Variables|/Game/Blueprint/Camera_BP.Camera_BP_C|Getlock_on_target (Variables|Default|Getfollow_cam)) _array_element)
      (bind _returnvalue (Collision|LineTraceByChannel (LocalVariables|Getsocket_location) (Transformation|GetActorLocation _array_element) "TraceTypeQuery1" false _outactors "None"))
      (if (not _returnvalue)
        (Utilities|IsValid (Variables|/Game/Blueprint/Character/BP_BaseEnemy.BP_BaseEnemy_C|GetLockOnMarker _array_element)
          (:Is%20Valid
            (if (> (Math|Vector|DotProduct (Math|Vector|Normalize (Math|Vector|GetForwardVector (Math|Rotator|FindLookatRotation (LocalVariables|Getsocket_location) (Transformation|GetActorLocation _array_element)))) (Math|Vector|Normalize (Math|Vector|GetForwardVector (LocalVariables|Getsocket_rotation)))) 0.6)
              (if (> (* (.Yaw (Math|Vector|GetYawPitchfromVector (Math|Vector|UnrotateVector (- (Math|Vector|GetForwardVector (Math|Rotator|FindLookatRotation (LocalVariables|Getsocket_location) (Transformation|GetActorLocation _array_element))) (Math|Vector|GetForwardVector (LocalVariables|Getsocket_rotation))) (LocalVariables|Getsocket_rotation)))) direction) 1e+01)
                (if (> (Math|Vector|DotProduct (Math|Vector|Normalize (Math|Vector|GetForwardVector (Math|Rotator|FindLookatRotation (LocalVariables|Getsocket_location) (Transformation|GetActorLocation _array_element)))) (Math|Vector|Normalize (Math|Vector|GetForwardVector (LocalVariables|Getsocket_rotation)))) (LocalVariables|Getmin_angle))
                  (LocalVariables|Setmin_angle (Math|Vector|DotProduct (Math|Vector|Normalize (Math|Vector|GetForwardVector (Math|Rotator|FindLookatRotation (LocalVariables|Getsocket_location) (Transformation|GetActorLocation _array_element)))) (Math|Vector|Normalize (Math|Vector|GetForwardVector (LocalVariables|Getsocket_rotation)))))
                  (LocalVariables|Setlock_on_target _array_element)))))))))
  (return (LocalVariables|Getlock_on_target)))

(fn GetLockonTarget
  (return (Variables|/Game/Blueprint/Camera_BP.Camera_BP_C|Getlock_on_target (Variables|Default|Getfollow_cam))))

(fn IsLockonTarget
  (params (actor :type Actor%20Object%20Reference))
  (return (== actor (Variables|/Game/Blueprint/Camera_BP.Camera_BP_C|Getlock_on_target (Variables|Default|Getfollow_cam)))))