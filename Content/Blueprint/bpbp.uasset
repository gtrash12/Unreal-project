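; Actor Blueprint (bpbp) that handles facing, look angles and target tracking, plus visibility toggles for a lock-on marker and state bar.
; RotateActorTimeline stops RotateLastInputTimeline, then turns the actor to a given rotation with an ExpoOut-eased timeline.
; Look snaps actor yaw toward a valid TargetActor and interpolates clamped LookPitch and LookYaw toward LookLocation.
; BeginPlay and Tick are disabled, so nothing in this graph calls Look.
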(event EventBeginPlay
  (|CallParentFunction) ; 지금 이 노드는 비활성 상태입니다. \n핀을 끌어서 다른 노드를 연결하면 활성화됩니다.
)

(event Collision|EventActorBeginOverlap
  (params (OtherActor :type Actor%20Object%20Reference)))

(event EventTick
  (params (DeltaSeconds :type Float%20%28single-precision%29))
  (|CallParentFunction DeltaSeconds) ; 지금 이 노드는 비활성 상태입니다. \n핀을 끌어서 다른 노드를 연결하면 활성화됩니다.
)

(event EventRotateActorTimeline
  (params (target_rotation :type Rotator :default "0, 0, 0") (time :type Float%20%28single-precision%29))
  (bind _rotatelastinputtimeline (Variables|Default|GetRotateLastInputTimeline))
  (bind _output_get (Variables|Default|Settmp_rotation (Transformation|GetActorRotation)))
  (Audio|Components|Audio|Stop _rotatelastinputtimeline)
  (Components|Timeline|SetPlayRate _rotatelastinputtimeline (/ 1.0 time))
  (bind _새_트랙_0 (Timeline|타임라인_1_0 PlayFromStart)
    (:Update
      (Transformation|SetActorRotation (Math|Interpolation|Ease "ExpoOut" _새_트랙_0 _output_get target_rotation true) true))))

(event EventLook
  (bind _target_actor (Variables|Default|Gettarget_actor)
    (:then
      (Variables|Default|Setlook_location (Transformation|GetActorLocation _target_actor))
      (Transformation|SetActorRotation (Math|Rotator|MakeRotator 0.0 0.0 (.Yaw (Math|Rotator|BreakRotator (Math|Rotator|FindLookatRotation (Transformation|GetActorLocation) (Variables|Default|Getlook_location)))))))
    (:else
      _))
  (Variables|Default|Setlook_pitch (Math|Float|ClampAngle (.Pitch (Math|Rotator|BreakRotator (Math|Interpolation|RInterpTo (Math|Rotator|MakeRotator 0.0 (Variables|Default|Getlook_pitch) (Variables|Default|Getlook_yaw)) (Math|Rotator|Delta(Rotator) (Math|Rotator|FindLookatRotation (Transformation|GetActorLocation) (Variables|Default|Getlook_location)) (Transformation|GetActorRotation)) (Utilities|Time|GetWorldDeltaSeconds) 3.0))) -9e+01 9e+01))
  (Variables|Default|Setlook_yaw (Math|Float|ClampAngle (.Yaw (Math|Rotator|BreakRotator (Math|Interpolation|RInterpTo (Math|Rotator|MakeRotator 0.0 (Variables|Default|Getlook_pitch) (Variables|Default|Getlook_yaw)) (Math|Rotator|Delta(Rotator) (Math|Rotator|FindLookatRotation (Transformation|GetActorLocation) (Variables|Default|Getlook_location)) (Transformation|GetActorRotation)) (Utilities|Time|GetWorldDeltaSeconds) 3.0))) -9e+01 9e+01)))

(event EventSetLookLocation
  (params (target_location :type Vector :default "0, 0, 0"))
  (Variables|Default|Setlook_location target_location))

(event EventSetLockonMarker
  (params (onoff :type Boolean))
  (Rendering|SetVisibility (Variables|Default|GetLockOnMarker) onoff false))

(event EventSetStateBarVisibility
  (params (onoff :type Boolean))
  (Rendering|SetVisibility (Variables|Default|GetStatebar) onoff false))

(event EventSetTarget
  (params (target :type Actor%20Object%20Reference))
  (Variables|Default|Settarget_actor target))

(fn ConstructionScript
  (|CallParentFunction))

(fn GetTarget
  (return (Variables|Default|Gettarget_actor)))