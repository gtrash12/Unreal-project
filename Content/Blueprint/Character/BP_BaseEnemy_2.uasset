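; BP_BaseEnemy_2 is an enemy character Blueprint that adds a health bar and lock-on marker to behavior inherited from its parent.
; On BeginPlay it binds the StateBar widget to itself, then applies WalkSpeed, so the speed depends on that widget cast succeeding.
; SetLockonMarker toggles marker visibility, while multicast damage simply forwards to the parent.
; Hit decal, blood effect and smoothed look-at rotation logic remain but are disconnected.
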(event EventBeginPlay
  (bind _state_bar (Variables|Default|Getstate_bar))
  ;[1 0.9656 0.6646] init
  (|CallParentFunction)
  (Utilities|IsValid _state_bar
    (:Is%20Valid
      (bind _aswidget_enemy_health_bar (Utilities|Casting|CastToWidget_EnemyHealthBar (UserInterface|GetWidget _state_bar)))
      (Default|Init _aswidget_enemy_health_bar self)
      (Variables|/Script/Engine.CharacterMovementComponent|SetMaxWalkSpeed (Variables|Character|GetCharacterMovement) (Variables|Default|Getwalk_speed)))))

(event EventApplyDamageMulticastExec
  (params (__target_damage_id :type Name :default "None") (damage_causer :type Actor%20Object%20Reference) (__hit_bone_name :type Name :default "None") (__hit_location :type Vector :default "0, 0, 0"))
  (|CallParentFunction __target_damage_id damage_causer __hit_bone_name __hit_location))

(event EventSetLockonMarker
  (params (__is_lock_on :type Boolean))
  (bind _lockonmarker (Variables|Default|GetLockOnMarker))
  ;[1 1 1] UI
  (Utilities|IsValid _lockonmarker
    (:Is%20Valid
      (Rendering|SetVisibility _lockonmarker __is_lock_on false))))

(fn ConstructionScript
  (|CallParentFunction))