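; BP_Boss is a boss character Blueprint that builds on a parent class for its core behavior.
; On BeginPlay it registers hand, foot and earthquake components by name in the AttackCollisions map.
; Death runs the parent logic, then plays a monster pain sound at the boss's location.
; Tick and the construction script only call the parent, and the overlap event is empty.
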(event EventBeginPlay
  (bind _attack_collisions (Variables|Default|Getattack_collisions))
  (|CallParentFunction)
  (Utilities|Map|Add _attack_collisions "left_hand" (Variables|Default|Getlefthand))
  (Utilities|Map|Add _attack_collisions "earthquake" (Variables|Default|Getearthquake))
  (Utilities|Map|Add _attack_collisions "left_foot" (Variables|Default|Getleftfoot))
  (Utilities|Map|Add _attack_collisions "right_hand" (Variables|Default|Getrighthand)))

(event Collision|EventActorBeginOverlap
  (params (OtherActor :type Actor%20Object%20Reference)))

(event EventTick
  (params (DeltaSeconds :type Float%20%28single-precision%29))
  (|CallParentFunction DeltaSeconds))

(event EventDeath
  (|CallParentFunction)
  (Audio|PlaySoundatLocation "/Game/SFX/monster/MONSTER_Pain_03_mono.MONSTER_Pain_03_mono" (Transformation|GetActorLocation) "0, 0, 0" 1.0 1.0 0.0 0 0 0))

(fn ConstructionScript
  (|CallParentFunction))