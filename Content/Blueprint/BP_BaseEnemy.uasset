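; Base enemy character with health bar, lock-on marker and target-facing look, extending a parent character that supplies state and damage handling.
; BT-facing events set target, look location and sprint, and play multicast attack montages turned toward the target.
; Damage retargets the enemy controller to the attacker, then shows the bar or triggers death with lock-on release, pelvis-down impulse and delayed destroy.
; Tick disables movement-facing during knockback and times ragdoll get-up.
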(event Custom|death
  (bind _returnvalue (Game|GetPlayerController 0))
  (bind _lockonmarker (Variables|Default|GetLockOnMarker))
  ;[1 1 1] Death process
  (Utilities|FlowControl|Sequence
    (:then_0
      (CallFunction|SetStateBarVisibility false)
      (bind _result (Class|InterfacePlayerController|IsLockonTarget(Message) _returnvalue self))
      (if _result
        (Class|InterfacePlayerController|ReleaseLockON(Message) _returnvalue)))
    (:then_1
      (Utilities|IsValid _lockonmarker
        (:Is%20Valid
          (Components|DestroyComponent _lockonmarker)
          (Components|DestroyComponent (Variables|Default|GetStatebar)))))
    (:then_2
      (Utilities|FlowControl|Delay 0.25)
      (Class|BaseCharacter|SetCharacterState "Death")
      (Class|SkeletalMeshComponent|AddImpulsetoAllBodiesBelow (Variables|Character|GetMesh) (+ (* (Transformation|GetVelocity) "10.000000,10.000000,3.000000") "0,0.000000,100.000000") "pelvis" false true)
      (Utilities|FlowControl|Delay 3.0)
      (Actor|DestroyActor))))

(event EventBeginPlay
  ;[1 1 1] init
  (|CallParentFunction)
  (bind _aswidget_enemy_health_bar (Utilities|Casting|CastToWidget_EnemyHealthBar (UserInterface|GetWidget (Variables|Default|GetStatebar))))
  (Default|Init _aswidget_enemy_health_bar self)
  (Variables|/Script/Engine.CharacterMovementComponent|SetMaxWalkSpeed (Variables|Character|GetCharacterMovement) (Variables|Default|Getwalk_speed)))

(event EventSetCharacterState
  (params (target_character_state :type ECharacterState%20Enum :default "Walk_and_Jump"))
  (|CallParentFunction target_character_state)
  (Variables|Default|Setdown_time 3.0))

(event EventTick
  (params (DeltaSeconds :type Float%20%28single-precision%29))
  (bind _charactermovement (Variables|Character|GetCharacterMovement))
  ;[1 1 1] tick
  (|CallParentFunction DeltaSeconds)
  (Utilities|FlowControl|Sequence
    (:then_0
      ;;[1 1 1] Set monster rotation to move direction when moving. when knock-back moving don't rotate monster
      (if (> (Variables|Default|Getknock_back_speed) 0.0)
        (Variables|/Script/Engine.CharacterMovementComponent|SetbOrientRotationToMovement _charactermovement false)
        (else
          (Variables|/Script/Engine.CharacterMovementComponent|SetbOrientRotationToMovement _charactermovement true))))
    (:then_1
      ;;[1 1 1] Get up Process wher monster down
      (switch Utilities|FlowControl|Switch|SwitchonECharacterState (Variables|Default|Getcharacter_state)
        (:Ragdoll
          (if (Variables|Default|Getis_ragdoll_on_the_ground)
            (bind _output_get (Variables|Default|Setdown_time (- (Variables|Default|Getdown_time) DeltaSeconds)))
            (if (<= _output_get 0.0)
              (Class|BaseCharacter|RagdollGetUp)
              (Class|BaseCharacter|SetCharacterState "Walk_and_Jump")
              (Variables|Default|Setis_on_sprint true))
            (else
              (Variables|Default|Setdown_time 2.0))))))))

(event EventApplyDamageMulticastExec
  (params (target_damage_data :type Damage%20Data%20Structure) (damage_causor :type Actor%20Object%20Reference))
  (bind _statebar (Variables|Default|GetStatebar))
  ;[1 1 1] Damage event override
  (|CallParentFunction target_damage_data damage_causor)
  (bind _output_get (Variables|Default|Settarget_actor damage_causor))
  (bind _ascontroller_enemy (Utilities|Casting|CastToController_Enemy (Pawn|GetController))
    (:then
      (Default|TargetChange _ascontroller_enemy _output_get))
    (:CastFailed
      _))
  (Utilities|IsValid _statebar
    (:Is%20Valid
      (Utilities|Casting|CastToWidget_EnemyHealthBar (UserInterface|GetWidget _statebar)))
    (:Is%20Not%20Valid
      _))
  (if (<= (Variables|Default|Gethp) 0.0)
    (CallFunction|Death)
    (else
      (CallFunction|SetStateBarVisibility true))))

(event EventSetLockonMarker
  (params (onoff :type Boolean))
  (bind _lockonmarker (Variables|Default|GetLockOnMarker))
  ;[1 1 1] UI
  (Utilities|IsValid _lockonmarker
    (:Is%20Valid
      (Rendering|SetVisibility _lockonmarker onoff false))))

(event EventSetStateBarVisibility
  (params (onoff :type Boolean))
  (bind _statebar (Variables|Default|GetStatebar))
  ;[1 1 1] UI
  (Utilities|IsValid _statebar
    (:Is%20Valid
      (Rendering|SetVisibility _statebar onoff false)
      (Widget|SetVisibility (UserInterface|GetWidget _statebar) "Visible"))))

(event Custom|AttackMulticast
  (params (last_movement_input :type Vector) (animation :type Anim%20Montage%20Object%20Reference))
  ;[1 1 1] attack event
  (Animation|PlayAnimMontage animation 1.0 "None")
  (Class|BaseCharacter|RotateActorwithinTime (Math|Rotator|MakeRotfromX last_movement_input) 0.4))

(event Custom|SprintMulticast
  (params (IsSprint :type Boolean))
  ;[1 1 1] character state relative
  (bind _output_get (Variables|Default|Setis_on_sprint IsSprint))
  (Variables|/Script/Engine.CharacterMovementComponent|SetMaxWalkSpeed (Variables|Character|GetCharacterMovement) (Math|Float|SelectFloat (Variables|Default|Getsprint_speed) (Variables|Default|Getwalk_speed) _output_get)))

(event EventSetLookRotation
  ;[1 1 1] Look func override
  (bind _target_actor (Variables|Default|Gettarget_actor)
    (:then
      (Variables|Default|Setlook_location (Transformation|GetActorLocation _target_actor)))
    (:else
      _))
  (Variables|Default|Setlook_pitch (Math|Float|ClampAngle (.Pitch (Math|Rotator|BreakRotator (Math|Interpolation|RInterpTo (Math|Rotator|MakeRotator 0.0 (Variables|Default|Getlook_pitch) (Variables|Default|Getlook_yaw)) (Math|Rotator|Delta(Rotator) (Math|Rotator|FindLookatRotation (Transformation|GetActorLocation) (Variables|Default|Getlook_location)) (Transformation|GetActorRotation)) (Utilities|Time|GetWorldDeltaSeconds) 3.0))) -9e+01 9e+01))
  (Variables|Default|Setlook_yaw (Math|Float|ClampAngle (.Yaw (Math|Rotator|BreakRotator (Math|Interpolation|RInterpTo (Math|Rotator|MakeRotator 0.0 (Variables|Default|Getlook_pitch) (Variables|Default|Getlook_yaw)) (Math|Rotator|Delta(Rotator) (Math|Rotator|FindLookatRotation (Transformation|GetActorLocation) (Variables|Default|Getlook_location)) (Transformation|GetActorRotation)) (Utilities|Time|GetWorldDeltaSeconds) 3.0))) -9e+01 9e+01)))

(event EventSetSprint
  (params (is_sprint :type Boolean))
  ;[1 1 1] character state relative
  (CallFunction|SprintMulticast is_sprint))

(event EventAttack
  (bind _returnvalue (Transformation|GetActorLocation))
  (bind _target_actor (Variables|Default|Gettarget_actor))
  (bind _returnvalue_2 (Transformation|GetActorLocation _target_actor))
  (bind _returnvalue_3 (Math|Rotator|FindLookatRotation _returnvalue _returnvalue_2))
  (bind _returnvalue_4 (Math|Vector|GetForwardVector _returnvalue_3))
  (bind (_x _y) (Math|Vector|BreakVector _returnvalue_4))
  ;[1 1 1] attack event
  (if (not (Class|AnimInstance|IsAnyMontagePlaying (Variables|Default|Getmain_anim_instance)))
    (switch Utilities|FlowControl|Switch|SwitchonECharacterState (Variables|Default|Getcharacter_state)
      (:Walk_and_Jump
        (CallFunction|AttackMulticast (Math|Vector|MakeVector _x _y 0.0) (Variables|Default|Getnext_attack_montage))))))

(event EventSetLookLocation
  (params (target_location :type Vector :default "0, 0, 0"))
  ;[1 1 1] character state relative
  (Variables|Default|Setlook_location target_location))

(event EventSetTarget
  (params (target :type Actor%20Object%20Reference))
  ;[1 1 1] character state relative
  (Variables|Default|Settarget_actor target))

(fn ConstructionScript
  (|CallParentFunction))

(fn GetAttackTraceChannel
  (return "TraceTypeQuery5"))

(fn GetTargetRotation
  (return (Math|Rotator|MakeRotator 0.0 0.0 (.Yaw (Math|Rotator|BreakRotator (Math|Rotator|FindLookatRotation (Transformation|GetActorLocation) (Variables|Default|Getlook_location)))))))

(fn GetTarget
  (return (Variables|Default|Gettarget_actor)))