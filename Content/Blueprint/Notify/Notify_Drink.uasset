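; Anim notify that applies the effects of the item being used when a drink animation reaches it, only for the local player pawn.
; It reads the inventory slot at the character's UsingItemIndex through the controller and looks up the item data in PWOGameInstance.
; Each listed effect runs on its class default object, with Value overwritten before ApplyItemEffectMessage is called, so no effect instances are created.
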(fn ReceivedNotify
  (params (MeshComp :type Skeletal%20Mesh%20Component%20Object%20Reference) (Animation :type Anim%20Sequence%20Base%20Object%20Reference))
  (bind _returnvalue (Components|GetOwner MeshComp))
  (if (== (Game|Player|GetPlayerPawn 0) _returnvalue)
    (bind _asbp_player_character_cpp (Utilities|Casting|CastToBP_PlayerCharacter_cpp _returnvalue))
    (bind _returnvalue_2 (Class|InterfacePlayerController|GetInventoryData(Message) (Pawn|GetController _asbp_player_character_cpp) (Variables|/Game/Blueprint/Character/BP_PlayerCharacter_cpp.BP_PlayerCharacter_cpp_C|Getusing_item_index _asbp_player_character_cpp)))
    (bind _aspwogame_instance (Utilities|Casting|CastToPWOGameInstance (Game|GetGameInstance)))
    (bind _returnvalue_3 (Class|PWOGameInstance|FindItemData _aspwogame_instance (.item_id (Utilities|Struct|BreakInventoryData _returnvalue_2))))
    (for _array_element (.item_effect_list (Utilities|Struct|BreakItemData _returnvalue_3))
      (bind _returnvalue_4 (Class|CustomBPFunctionLibrary|GetClassDefaultObject (.item_effect (Utilities|Struct|BreakItemEffect _array_element))))
      (Variables|/Script/CyperArena.BaseItemEffect|Setvalue _returnvalue_4 (.value (Utilities|Struct|BreakItemEffect _array_element)))
      (Class|InterfaceItemEffect|ApplyItemEffect(Message) _returnvalue_4 _asbp_player_character_cpp (Variables|/Game/Blueprint/Character/BP_PlayerCharacter_cpp.BP_PlayerCharacter_cpp_C|Getusing_item_index _asbp_player_character_cpp)))
    (return true)))