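; Interactable loot chest that shows a HUD prompt and, on Interact, opens and destroys its Box component.
; If locked, a one-time timed sequence plays animations, optional effects and sounds, then swings the lid open with optional light fade-in.
; That sequence also drops items server-side through a delayed-loop macro, randomizing each item's yaw, distance and jump.
; If already unlocked, it only plays the lid timeline; the close-and-unlock logic is unconnected.
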(event OnComponentEndOverlap(Box)
  (params (OverlappedComponent :type Primitive%20Component%20Object%20Reference) (OtherActor :type Actor%20Object%20Reference) (OtherComp :type Primitive%20Component%20Object%20Reference) (OtherBodyIndex :type Integer))
  ;[1 1 1] Open and Close if Unlocked
  (if (Variables|Default|GetisUnlocked)
    (bind _cme_open (Timeline|Open%20and%20Close%20Unlocked Reverse)
      (:Update
        (Transformation|SetRelativeRotation (Variables|Default|GetSM_Lid) (Math|Rotator|MakeRotator _cme_open 0.0 0.0) false false)))))

(event Custom|Open
  (bind _arrow (Variables|Default|GetArrow))
  (bind _sm_base (Variables|Default|GetSM_Base))
  (bind _returnvalue (Transformation|GetWorldLocation _sm_base))
  (if (Variables|Default|GetisUnlocked)
    ;[1 1 1] Open and Close if Unlocked
    (Audio|PlaySoundatLocation "/Game/Heroic_Chests_Volume_1/Audio/ECV1_Common_Clasp_Cue.ECV1_Common_Clasp_Cue" (Transformation|GetWorldLocation (Variables|Default|GetSM_Base)) "0, 0, 0" 1.0 1.0 0.0 "/Game/Heroic_Chests_Volume_1/Audio/Attenuation_Basic_SA.Attenuation_Basic_SA" 0 0)
    (bind _cme_open (Timeline|Open%20and%20Close%20Unlocked Play)
      (:Update
        (Transformation|SetRelativeRotation (Variables|Default|GetSM_Lid) (Math|Rotator|MakeRotator _cme_open 0.0 0.0) false false)))
    (else
      ;[1 1 1] Implement User Variables
      (Utilities|FlowControl|DoOnce false
        (:Completed
          (Audio|PlaySoundatLocation "/Game/Heroic_Chests_Volume_1/Audio/ECV2_Common_Diagetic_Cue.ECV2_Common_Diagetic_Cue" _returnvalue "0, 0, 0" 1.0 1.0 0.0 "/Game/Heroic_Chests_Volume_1/Audio/Attenuation_Basic_SA.Attenuation_Basic_SA" 0 0)
          (if (Variables|Default|GetEthereal)
            (Audio|PlaySoundatLocation "/Game/Heroic_Chests_Volume_1/Audio/ECV2_Common_Ethereal_Cue.ECV2_Common_Ethereal_Cue" _returnvalue "0, 0, 0" 0.4 1.0 0.0 "/Game/Heroic_Chests_Volume_1/Audio/Attenuation_Basic_SA.Attenuation_Basic_SA" 0 0)
            (Utilities|FlowControl|Delay 0.0))
          (Components|Animation|PlayAnimation (Variables|Default|GetSKM_Animation_A) "/Game/Heroic_Chests_Volume_1/Animations/ECV2_Common_Anim.ECV2_Common_Anim" false)
          (Utilities|FlowControl|Delay 0.5)
          (Components|Animation|PlayAnimation (Variables|Default|GetSKM_Animation_B) "/Game/Heroic_Chests_Volume_1/Animations/ECV2_Common_Anim.ECV2_Common_Anim" false)
          (Utilities|FlowControl|Delay 6.0)
          (if (Variables|Default|Getparticles)
            (Effects|SpawnEmitteratLocation "/Game/Heroic_Chests_Volume_1/Particles/ECV2_Common_P.ECV2_Common_P" (Transformation|GetWorldLocation _arrow) (Transformation|GetWorldRotation _arrow) "1.000000,1.000000,1.000000" false))
          (Utilities|FlowControl|Delay 1.0)
          (if (Variables|Default|GetMelodic)
            (Audio|PlaySoundatLocation "/Game/Heroic_Chests_Volume_1/Audio/ECV1_Common_Melodic_Cue.ECV1_Common_Melodic_Cue" (Transformation|GetActorLocation) "0, 0, 0" 1.0 1.0 0.0 "/Game/Heroic_Chests_Volume_1/Audio/Attenuation_Basic_SA.Attenuation_Basic_SA" 0 0))
          (CallFunction|Dropitem)
          ;[1 1 1] Open Lid
          (bind (_direction _cme_open_2 _lightintensity) (Timeline|Open_Lid PlayFromStart)
            (:Update
              (Transformation|SetRelativeRotation (Variables|Default|GetSM_Lid) (Math|Rotator|MakeRotator _cme_open_2 0.0 0.0) false false)
              (if (Variables|Default|Getlight)
                (Rendering|Components|Light|SetIntensity (Variables|Default|GetPointLight) (Math|Float|Lerp 0.0 (Variables|Default|GetIntensity) _lightintensity))
                (Utilities|FlowControl|DoOnce false
                  (:Completed
                    (Audio|PlaySoundatLocation "/Game/Heroic_Chests_Volume_1/Audio/ECV1_Common_Clasp_Cue.ECV1_Common_Clasp_Cue" (Transformation|GetWorldLocation (Variables|Default|GetSM_Base)) "0, 0, 0" 1.0 1.0 0.0 "/Game/Heroic_Chests_Volume_1/Audio/Attenuation_Basic_SA.Attenuation_Basic_SA" 0 0)))))))))))

(event Custom|dropitem
  (bind _returnvalue (Transformation|GetActorRotation))
  (if (Networking|IsServer)
    (Utilities|ForLoopwithDelay 1 (Variables|Default|Getdropitemcount) 0.1
      (:loop%20body
        (bind _returnvalue_2 (Game|SpawnActorfromClass "/Game/Blueprint/Interactable/DropItem.DropItem_C" (Math|Transform|MakeTransform (Transformation|GetActorLocation) (Math|Rotator|MakeRotator (.roll _returnvalue) (.pitch _returnvalue) (+ (.yaw _returnvalue) (Math|Random|RandomFloatinRange -145.0 -45.0))) "1,1,1") "Undefined" 0 0))
        (Variables|/Game/Blueprint/Interactable/DropItem.DropItem_C|Setdistance _returnvalue_2 (Math|Random|RandomFloatinRange 1.2e+02 3e+02))
        (Variables|/Game/Blueprint/Interactable/DropItem.DropItem_C|Setjump _returnvalue_2 (Math|Random|RandomFloatinRange 1e+02 3e+02))))))

(event EventInteract
  (params (causer :type Actor%20Object%20Reference))
  (bind _box (Variables|Default|GetBox))
  (CallFunction|Open)
  (Utilities|IsValid _box
    (:Is%20Valid
      (Components|DestroyComponent _box))))

(event EventPopInteractionInfo
  (params (causer :type Actor%20Object%20Reference))
  (bind _ascontroller_player_character_cpp_2 (Utilities|Casting|CastToController_PlayerCharacter_cpp_2 (Game|GetPlayerController 0)))
  (Utilities|IsValid (Variables|/Game/Blueprint/controller/Controller_PlayerCharacter_cpp_2.Controller_PlayerCharacter_cpp_2_C|GetHUD_reference _ascontroller_player_character_cpp_2)
    (:Is%20Valid
      (Rendering|Components|TextRender|SetText (Variables|/Game/Blueprint/Widget/Widget_UI.Widget_UI_C|Gettext_left (Variables|/Game/Blueprint/controller/Controller_PlayerCharacter_cpp_2.Controller_PlayerCharacter_cpp_2_C|GetHUD_reference _ascontroller_player_character_cpp_2)) "F : 열기")
      (Widget|SetVisibility (Variables|/Game/Blueprint/Widget/Widget_UI.Widget_UI_C|GetInteractBox (Variables|/Game/Blueprint/controller/Controller_PlayerCharacter_cpp_2.Controller_PlayerCharacter_cpp_2_C|GetHUD_reference _ascontroller_player_character_cpp_2)) "Visible"))))

(event EventRemoveInteractionInfo
  (params (causer :type Actor%20Object%20Reference))
  (bind _ascontroller_player_character_cpp_2 (Utilities|Casting|CastToController_PlayerCharacter_cpp_2 (Game|GetPlayerController 0)))
  (Utilities|IsValid (Variables|/Game/Blueprint/controller/Controller_PlayerCharacter_cpp_2.Controller_PlayerCharacter_cpp_2_C|GetHUD_reference _ascontroller_player_character_cpp_2)
    (:Is%20Valid
      (Widget|SetVisibility (Variables|/Game/Blueprint/Widget/Widget_UI.Widget_UI_C|GetInteractBox (Variables|/Game/Blueprint/controller/Controller_PlayerCharacter_cpp_2.Controller_PlayerCharacter_cpp_2_C|GetHUD_reference _ascontroller_player_character_cpp_2)) "Hidden"))))

(fn ConstructionScript
  (bind _pointlight (Variables|Default|GetPointLight))
  (Rendering|Components|Light|SetLightColor _pointlight (Variables|Default|GetLight%20Color) true)
  (Rendering|Components|Light|SetIntensity _pointlight 0.0)
  (if (Variables|Default|GetInterior)
    (Rendering|SetVisibility (Variables|Default|GetSM_Base_Interior) true false)
    (Rendering|SetVisibility (Variables|Default|GetSM_Lid_Interior) true false)))