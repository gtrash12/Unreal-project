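; DropItem is an interactable pickup that pops out when spawned and grants the player a potion.
; On BeginPlay it plays a spawn sound and a Pop timeline moves it along an arced hop using swept location updates.
; Interaction events toggle the HUD pickup prompt on the first player controller.
; Picking it up plays a sound, then, when the causer has authority, increments that controller's potion count and destroys the actor after a short delay.
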(event Custom|poping
  (bind _returnvalue (Transformation|GetActorLocation))
  (Audio|PlaySoundatLocation "/Game/SFX/SFX/MAGIC_SPELL_Spawn_mono.MAGIC_SPELL_Spawn_mono" _returnvalue "0, 0, 0" 1.0 1.0 0.0 "/Game/Heroic_Chests_Volume_1/Audio/Attenuation_Basic_SA.Attenuation_Basic_SA" 0 0)
  (bind _output_get (Variables|Default|Setstart_location _returnvalue))
  (bind (_direction _distance _jump) (Timeline|pop PlayFromStart)
    (:Update
      (Transformation|SetActorLocation (+ _output_get (* (Transformation|GetActorForwardVector) (* _distance (Variables|Default|Getdistance))) (* (Transformation|GetActorUpVector) (* _jump (Variables|Default|Getjump)))) true false))))

(event EventPopInteractionInfo
  (params (causor :type Actor%20Object%20Reference))
  (bind _ascontroller_player_character_cpp (Utilities|Casting|CastToController_PlayerCharacter_cpp (Game|GetPlayerController 0)))
  (Utilities|IsValid (Variables|/Game/Blueprint/controller/Controller_PlayerCharacter_cpp.Controller_PlayerCharacter_cpp_C|GetHUD_reference _ascontroller_player_character_cpp)
    (:Is%20Valid
      (Rendering|Components|TextRender|SetText (Variables|/Game/Blueprint/Widget/Widget_UI.Widget_UI_C|Gettext_left (Variables|/Game/Blueprint/controller/Controller_PlayerCharacter_cpp.Controller_PlayerCharacter_cpp_C|GetHUD_reference _ascontroller_player_character_cpp)) "F : 줍기")
      (Widget|SetVisibility (Variables|/Game/Blueprint/Widget/Widget_UI.Widget_UI_C|GetInteractBox (Variables|/Game/Blueprint/controller/Controller_PlayerCharacter_cpp.Controller_PlayerCharacter_cpp_C|GetHUD_reference _ascontroller_player_character_cpp)) "Visible"))))

(event EventInteraction
  (params (causor :type Actor%20Object%20Reference))
  (Class|InterfaceGeneral|RemoveInteractionInfo)
  (Audio|PlaySoundatLocation "/Game/SFX/SFX/PUZZLE_Success_Harp_Three_Note_Bright_End_Wet_stereo.PUZZLE_Success_Harp_Three_Note_Bright_End_Wet_stereo" (Transformation|GetActorLocation) "0, 0, 0" 1.0 1.0 0.0 0 0 0)
  (if (Ability|HasAuthority causor)
    (bind _asbase_character (Utilities|Casting|CastToBaseCharacter causor))
    (bind _ascontroller_player_character_cpp (Utilities|Casting|CastToController_PlayerCharacter_cpp (Pawn|GetController _asbase_character)))
    (Math|Integer|IncrementInt (Variables|/Game/Blueprint/controller/Controller_PlayerCharacter_cpp.Controller_PlayerCharacter_cpp_C|Getpotion_count _ascontroller_player_character_cpp)
      (:%20%20
        (Utilities|FlowControl|Delay 0.1)
        (Utilities|IsValid self
          (:Is%20Valid
            (Actor|DestroyActor)))))))

(event EventBeginPlay
  (CallFunction|Poping))

(event EventRemoveInteractionInfo
  (params (causor :type Actor%20Object%20Reference))
  (bind _ascontroller_player_character_cpp (Utilities|Casting|CastToController_PlayerCharacter_cpp (Game|GetPlayerController 0)))
  (Utilities|IsValid (Variables|/Game/Blueprint/controller/Controller_PlayerCharacter_cpp.Controller_PlayerCharacter_cpp_C|GetHUD_reference _ascontroller_player_character_cpp)
    (:Is%20Valid
      (Widget|SetVisibility (Variables|/Game/Blueprint/Widget/Widget_UI.Widget_UI_C|GetInteractBox (Variables|/Game/Blueprint/controller/Controller_PlayerCharacter_cpp.Controller_PlayerCharacter_cpp_C|GetHUD_reference _ascontroller_player_character_cpp)) "Hidden"))))

(fn ConstructionScript)