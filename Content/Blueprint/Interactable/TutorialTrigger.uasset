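; TutorialTrigger is an interactable Blueprint that shows a tutorial message on the player's HUD.
; PopInteractionInfo gets player 0's Controller_PlayerCharacter_cpp, writes TutorialMessage into the HUD's TextLeft and makes InteractBox visible.
; RemoveInteractionInfo hides that InteractBox again, and both events act only when the controller cast succeeds and the HUD reference is valid.
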(event EventPopInteractionInfo
  (params (causor :type Actor%20Object%20Reference))
  (bind _ascontroller_player_character_cpp (Utilities|Casting|CastToController_PlayerCharacter_cpp (Game|GetPlayerController 0)))
  (Utilities|IsValid (Variables|/Game/Blueprint/controller/Controller_PlayerCharacter_cpp.Controller_PlayerCharacter_cpp_C|GetHUD_reference _ascontroller_player_character_cpp)
    (:Is%20Valid
      (Rendering|Components|TextRender|SetText (Variables|/Game/Blueprint/Widget/Widget_UI.Widget_UI_C|Gettext_left (Variables|/Game/Blueprint/controller/Controller_PlayerCharacter_cpp.Controller_PlayerCharacter_cpp_C|GetHUD_reference _ascontroller_player_character_cpp)) (Variables|Default|Gettutorial_message))
      (Widget|SetVisibility (Variables|/Game/Blueprint/Widget/Widget_UI.Widget_UI_C|GetInteractBox (Variables|/Game/Blueprint/controller/Controller_PlayerCharacter_cpp.Controller_PlayerCharacter_cpp_C|GetHUD_reference _ascontroller_player_character_cpp)) "Visible"))))

(event EventRemoveInteractionInfo
  (params (causor :type Actor%20Object%20Reference))
  (bind _ascontroller_player_character_cpp (Utilities|Casting|CastToController_PlayerCharacter_cpp (Game|GetPlayerController 0)))
  (Utilities|IsValid (Variables|/Game/Blueprint/controller/Controller_PlayerCharacter_cpp.Controller_PlayerCharacter_cpp_C|GetHUD_reference _ascontroller_player_character_cpp)
    (:Is%20Valid
      (Widget|SetVisibility (Variables|/Game/Blueprint/Widget/Widget_UI.Widget_UI_C|GetInteractBox (Variables|/Game/Blueprint/controller/Controller_PlayerCharacter_cpp.Controller_PlayerCharacter_cpp_C|GetHUD_reference _ascontroller_player_character_cpp)) "Hidden"))))

(fn ConstructionScript)