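; Follow camera actor with a spring arm that tracks the target character's camera socket and normally matches its control rotation.
; Each tick, a rightward camera-channel trace sets a sideways offset to keep the camera inside walls, cleared once via DoOnce when unblocked.
; At high target speed without mouse or left-stick input, it eases toward looking at the character and overwrites control rotation.
; Debug drawing shows the trace and arm.
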(event EventTick
  (params (DeltaSeconds :type Float%20%28single-precision%29))
  (bind _returnvalue (Game|GetPlayerController 0))
  (bind _target (Variables|Default|GetTarget))
  (bind _camera (Variables|Default|GetCamera))
  (bind _target_2 (Variables|Default|GetTarget))
  (bind _target_3 (Variables|Default|GetTarget))
  (bind _camera_2 (Variables|Default|GetCamera))
  (bind _springarm (Variables|Default|GetSpringArm))
  (bind _returnvalue_2 (Transformation|GetWorldLocation _camera))
  (bind (_stickx _sticky) (Class|PlayerController|GetInputAnalogStickState _returnvalue "CAS_LeftStick"))
  (bind _returnvalue_3 (Transformation|GetActorLocation _target_2))
  (bind (_deltax _deltay) (Class|PlayerController|GetInputMouseDelta _returnvalue))
  (bind _returnvalue_4 (Transformation|GetActorLocation _target))
  (bind _returnvalue_5 (Transformation|GetWorldLocation _springarm))
  (bind _returnvalue_6 (Transformation|GetWorldLocation _camera_2))
  (bind _returnvalue_7 (Math|Rotator|FindLookatRotation _returnvalue_2 _returnvalue_4))
  (bind _returnvalue_8 (+ _returnvalue_3 "0, 0,50.000000"))
  (Utilities|FlowControl|Sequence
    (:then_0
      ;[1 1 1] 카메라 벽 밖으로 안나가게
      (bind (_outhit _returnvalue_9) (Collision|LineTraceByChannel _returnvalue_8 (+ (* (Math|Vector|GetRightVector (Transformation|GetWorldRotation (Variables|Default|GetSpringArm))) 6e+01) _returnvalue_8) "TraceTypeQuery2" false 0 "ForOneFrame"))
      (if (and _returnvalue_9 (.bBlockingHit (Collision|BreakHitResult _outhit)))
        (Variables|Default|Setlocation_offset (Math|Vector|MakeVector 0.0 (- (Math|Vector|Distance(Vector) (.Location (Collision|BreakHitResult _outhit)) _returnvalue_8) 6e+01) 0.0))
        (goto _label Reset)
        (else
          (Utilities|FlowControl|DoOnce true :!label _label
            (:Completed
              (Variables|Default|Setlocation_offset (Math|Vector|MakeVector 0.0 0.0 0.0)))))))
    (:then_1
      (Transformation|SetActorLocation (+ (Transformation|GetSocketLocation (Variables|/Script/Engine.Character|GetMesh _target_3) "camera_following_socket") (* (Math|Vector|GetRightVector (Transformation|GetActorRotation _target_3)) (.y (Variables|Default|Getlocation_offset)))) false false)
      (if (< (Math|Vector|VectorLength (Transformation|GetVelocity (Variables|Default|GetTarget))) 2e+03)
        (Transformation|SetActorRotation (Pawn|GetControlRotation (Variables|Default|GetTarget) :!class /Script/Engine.Pawn) :!label _label_2)
        (elif (Math|Boolean|ANDBoolean (== _deltax 0.0) (== _deltay 0.0) (== _stickx 0.0) (== _sticky 0.0))
          ;[1 1 1] 캐릭터 속도 임계치 초과시 컨트롤 로테이션이 아니라 캐릭터를 바라보는 방향으로 카메라 보간 후 컨트롤 로테이션을 맞춤
          (Transformation|SetActorRotation (Math|Interpolation|RInterpTo (Transformation|GetActorRotation) _returnvalue_7 DeltaSeconds 2.5))
          (Pawn|SetControlRotation (Game|GetPlayerController 0) _returnvalue_7)
          (else
            (goto _label_2)))))
    (:then_2
      (Rendering|Debug|DrawDebugPoint _returnvalue_6 1e+01 "(R=1.000000,G=0.000000,B=0.000000,A=1.000000)" 0.0)
      (Rendering|Debug|DrawDebugPoint _returnvalue_5 1e+01 "(R=0.005102,G=1.000000,B=0.000000,A=1.000000)" 0.0)
      (Rendering|Debug|DrawDebugLine _returnvalue_5 _returnvalue_6 "(R=0.819650,G=0.000000,B=1.000000,A=1.000000)" 0.0 0.0))))

(fn ConstructionScript)